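; BP_Menu3D is an actor for a 3D menu screen that moves the player's view to other linked menu actors.
; On BeginPlay it binds to the transition dispatcher of its WB_Menu3DWidget, which supplies an index into LinkedMenus.
; A valid index disables this actor's collision, enables the target's, and eases the player's view target to that menu with SetViewTargetWithBlend.
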(event Custom|TransitionTo
  (params (NewMenu :type BP%20Menu%203D%20Object%20Reference))
  (Collision|SetActorEnableCollision false)
  (Collision|SetActorEnableCollision NewMenu true)
  (Game|Player|SetViewTargetwithBlend (Game|GetPlayerController 0) NewMenu 2.0 "VTBlend_EaseInOut" 2.3 false))

(event Custom|TransitionToLinkedMenu_Event
  (params (MenuIndex :type Integer))
  (if (Utilities|Array|IsValidIndex (Variables|Default|GetLinkedMenus) MenuIndex)
    (CallFunction|Transitionto (Utilities|Array|Get(acopy) (Variables|Default|GetLinkedMenus) MenuIndex))))

(event EventBeginPlay
  (bind _aswb_menu_3dwidget (Utilities|Casting|CastToWB_Menu3DWidget (UserInterface|GetUserWidgetObject (Variables|Default|GetWidget))))
  (EventDispatchers|AssignTransitiontoLinkedMenu _aswb_menu_3dwidget (delegate Custom|TransitionToLinkedMenu_Event)))

(fn ConstructionScript)