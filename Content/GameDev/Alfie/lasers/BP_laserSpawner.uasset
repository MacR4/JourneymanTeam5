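; BP_laserSpawner is a rotatable laser emitter that spawns a BP_laser at its Arrow's location, facing along the actor's rotation.
; On activation it binds to the begin and end rotation events and spawns the first laser, passing its display name as the laser ID along with its colour.
; The child laser is destroyed when rotation begins and respawned when rotation ends, rather than being updated during the turn.
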(event Custom|activate_Event
  (EventDispatchers|BindEventtoEndRotation (delegate Custom|end%20rotation_Event))
  (EventDispatchers|BindEventtoBeginRotation (delegate Custom|begin%20rotation_Event))
  (bind _output_get (Variables|Default|SetID (Utilities|GetDisplayName self)))
  (bind _returnvalue (Game|SpawnActorfromClass "/Game/GameDev/Alfie/lasers/BP_laser.BP_laser_C" (Math|Transform|MakeTransform (Transformation|GetWorldLocation (Variables|Default|GetArrow)) (Transformation|GetActorRotation) "1.000000,1.000000,1.000000") "Undefined" "MultiplyWithRoot" self _output_get 0 (Variables|Default|GetLaserColour) 0 0))
  (Variables|Default|SetChild%20laser _returnvalue))

(event Custom|end%20rotation_Event
  (bind _output_get (Variables|Default|SetID (Utilities|GetDisplayName self)))
  (bind _returnvalue (Game|SpawnActorfromClass "/Game/GameDev/Alfie/lasers/BP_laser.BP_laser_C" (Math|Transform|MakeTransform (Transformation|GetWorldLocation (Variables|Default|GetArrow)) (Transformation|GetActorRotation) "1.000000,1.000000,1.000000") "Undefined" "MultiplyWithRoot" self _output_get 0 (Variables|Default|GetLaserColour) 0 0))
  (Variables|Default|SetChild%20laser _returnvalue))

(event Custom|begin%20rotation_Event
  (bind _child_laser (Variables|Default|GetChild%20laser))
  (Utilities|IsValid _child_laser
    (:Is%20Valid
      (Actor|DestroyActor _child_laser))))

(fn ConstructionScript
  (|CallParentFunction))