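; BP_laserTarget_Mushroom is a laser target that reveals its linked Target actors in game when a laser hits it.
; BeginPlay binds the hit event and applies the configured mesh to SMParent.
; LaserBounce records incoming lasers, skips any whose LaserId is already stored, and calls LaserHit for new ones.
; After that call, it clears the stored lasers if HitResponse is false.
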(event Custom|Laser%20hit_Event
  (for _array_element (Variables|Default|GetTarget)
    (Utilities|IsValid _array_element
      (:Is%20Valid
        (Rendering|SetActorHiddenInGame _array_element false)))))

(event EventBeginPlay
  (EventDispatchers|BindEventtoLaserHit (delegate Custom|Laser%20hit_Event))
  (Components|StaticMesh|SetStaticMesh (Variables|Default|GetSM_Parent) (Variables|Default|Getmesh)))

(fn ConstructionScript
  (|CallParentFunction))

(fn LaserBounce
  (params (Laser%20hit%20 :type BP%20Laser%20Object%20Reference) (Hit%20response :type Boolean) (Hit%20information :type Hit%20Result%20Structure))
  (bind _overlapping_actors (Variables|Default|GetOverlapping%20Actors))
  (bind _array_element (Utilities|Array|ForEachLoopwithBreak _overlapping_actors :!label _label)
    (:LoopBody
      (Utilities|IsValid _array_element
        (:Is%20Valid
          (bind _asbp_laser (Utilities|Casting|CastToBP_laser _array_element))
          (if (Utilities|Enum|Equal(Enum) (Variables|/Game/GameDev/Alfie/lasers/BP_laser.BP_laser_C|Getlaser%20id _asbp_laser) (Variables|/Game/GameDev/Alfie/lasers/BP_laser.BP_laser_C|Getlaser%20id Laser%20hit%20))
            (Variables|Default|SetIn%20array (Utilities|Enum|Equal(Enum) (Variables|/Game/GameDev/Alfie/lasers/BP_laser.BP_laser_C|Getlaser%20id _asbp_laser) (Variables|/Game/GameDev/Alfie/lasers/BP_laser.BP_laser_C|Getlaser%20id Laser%20hit%20)))
            (goto _label Break)))))
    (:Completed
      (if (not (Variables|Default|GetIn%20array))
        (Utilities|Array|Add _overlapping_actors Laser%20hit%20)
        (Default|CallLaserHit)
        (if Hit%20response
          (return 0)
          (else
            (Utilities|Array|Clear (Variables|Default|GetOverlapping%20Actors))))))))