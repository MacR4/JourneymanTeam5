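; Laser beam actor that extends along its up vector until it is blocked or reaches its Range.
; Each Tick it runs a small box trace on Visibility and scales the beam mesh parent and fireflies effect to the hit distance.
; Hit actors implementing BPI_lasers receive a LaserBounceMessage with the laser and hit info.
; ChangeColour is empty and CancelTargetHit only returns false.
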(event EventBeginPlay)

(event EventTick
  (params (DeltaSeconds :type Float%20%28single-precision%29))
  (CallFunction|SetEndPoint))

(fn ConstructionScript
  (|CallParentFunction))

(fn ChangeColour)

(fn SetEndPoint
  (bind _returnvalue (Transformation|GetActorLocation))
  (bind _returnvalue_2 (Transformation|GetActorUpVector))
  (bind _returnvalue_3 (* _returnvalue_2 2.0))
  (bind _returnvalue_4 (+ _returnvalue _returnvalue_3))
  (bind _outhit (Collision|BoxTraceByChannel _returnvalue_4 (+ _returnvalue_4 (* _returnvalue_2 (LocalVariables|GetRange))) "0.500000,0.500000,0.500000" "0, 0, 0" "TraceTypeQuery1" false (Variables|Default|GetActors%20to%20Ignore) "None"))
  (bind _output_get (LocalVariables|Sethit%20info _outhit))
  (LocalVariables|SetHit%20actor (.HitActor (Collision|BreakHitResult _output_get)))
  (Transformation|SetWorldScale3D (Variables|Default|GetSM_Parent) (Math|Vector|MakeVector 0.05 0.05 (Math|Float|SelectFloat (/ (+ (.Distance (Collision|BreakHitResult _output_get)) 1.0) 1e+02) (/ (LocalVariables|GetRange) 1e+02) (.bBlockingHit (Collision|BreakHitResult _output_get)))))
  (Transformation|SetWorldScale3D (Variables|Default|GetP_Fireflies) (Math|Vector|MakeVector 0.1 0.1 (Math|Float|SelectFloat (/ (+ (.Distance (Collision|BreakHitResult _output_get)) 1.0) 1e+02) (/ (LocalVariables|GetRange) 1e+02) (.bBlockingHit (Collision|BreakHitResult _output_get)))))
  (if (Utilities|DoesObjectImplementInterface (LocalVariables|GetHit%20actor) "/Game/GameDev/Alfie/lasers/BPI_lasers.BPI_lasers_C")
    (Class|BPILasers|LaserBounce(Message) (LocalVariables|GetHit%20actor) self true (LocalVariables|Gethit%20info))))

(fn CancelTargetHit
  (params (override :type Boolean))
  (Utilities|FlowControl|Sequence
    (:then_0
      (return false))))