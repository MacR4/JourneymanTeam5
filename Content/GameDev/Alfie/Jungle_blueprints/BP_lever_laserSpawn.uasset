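; Lever Blueprint for a jungle area that, going by its name, triggers a laser spawner.
; On BeginPlay it binds a handler to the lever activate event.
; The handler prints a debug string and calls ActivateEvent on its Spawner reference if the player character overlaps the Box.
; An unconnected, unfinished loop compares IDs against LeverID across Rotator_Parent actors and never runs.
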(event Custom|Lever%20activate_Event
  (Development|PrintString "Hello")
  (if (Collision|IsOverlappingActor (Variables|Default|GetBox) (Game|GetPlayerCharacter 0) :!class /Script/Engine.PrimitiveComponent)
    (Default|ActivateEvent (Variables|Default|Getspawner))))

(event EventBeginPlay
  (EventDispatchers|BindEventtoLeverActivate (delegate Custom|Lever%20activate_Event)))

(fn ConstructionScript)