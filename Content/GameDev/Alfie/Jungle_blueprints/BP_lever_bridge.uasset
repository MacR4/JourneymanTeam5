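; Lever actor that lowers a linked bridge when activated with the player nearby.
; On BeginPlay it binds a handler to the lever-activate event.
; The handler calls the lower-bridge function on its Bridge reference only if the player character overlaps its Box.
; A disconnected search of Rotator_Parent actors by LeverID never runs.
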(event Custom|Lever%20activate_Event
  (if (Collision|IsOverlappingActor (Variables|Default|GetBox) (Game|GetPlayerCharacter 0) :!class /Script/Engine.PrimitiveComponent)
    (Default|CallLowerBridge (Variables|Default|Getbridge))))

(event EventBeginPlay
  (EventDispatchers|BindEventtoLeverActivate (delegate Custom|Lever%20activate_Event)))

(fn ConstructionScript)