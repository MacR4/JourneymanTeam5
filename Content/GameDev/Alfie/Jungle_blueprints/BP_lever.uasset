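; BP_lever is a lever that rotates linked Rotator_Parent actors when activated with the player in range.
; On BeginPlay it binds to a LeverActivate event, which prints a debug string and checks whether the player character overlaps its Box.
; If so, it searches all Rotator_Parent actors and calls CallRotate on each whose ID matches LeverID.
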(event Custom|Lever%20activate_Event
  (Development|PrintString "Hello")
  (if (Collision|IsOverlappingActor (Variables|Default|GetBox) (Game|GetPlayerCharacter 0) :!class /Script/Engine.PrimitiveComponent)
    (bind _outactors (Actor|GetAllActorsOfClass "/Game/GameDev/Alfie/Rotator_Parent.Rotator_Parent_C"))
    (bind _array_element (Utilities|Array|ForEachLoopwithBreak _outactors)
      (:LoopBody
        (if (== (Variables|/Game/GameDev/Alfie/Rotator_Parent.Rotator_Parent_C|GetID _array_element) (Variables|Default|GetLever%20ID))
          (Default|CallRotate _array_element))))))

(event EventBeginPlay
  (EventDispatchers|BindEventtoLeverActivate (delegate Custom|Lever%20activate_Event)))

(fn ConstructionScript)