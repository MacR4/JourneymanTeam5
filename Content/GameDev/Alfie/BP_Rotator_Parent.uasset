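; Parent actor that rotates in 90-degree steps on a bound Rotate event and snaps to zero rotation on a bound reset event.
; Step direction depends on whether current yaw plus 90 stays within MaxStartRotation.
; A timeline lerps along the shortest path, with DoOnce gates blocking re-triggers mid-turn and notifying all BP_FinalSpawner actors once when rotation begins, then again when it ends.
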(event Custom|Rotate_Event
  (Utilities|FlowControl|DoOnce false :!label _label
    (:Completed
      (bind _output_get (Variables|Default|SetStarting%20Rotation_0 (Transformation|GetActorRotation self)))
      (Variables|Default|Setend%20rotation (Math|Rotator|CombineRotators _output_get (Math|Rotator|SelectRotator "0.000000,90.000000,0.000000" "0.000000,-90.000000,0.000000" (<= (+ (.yaw (Variables|Default|GetStarting%20Rotation_0)) 9e+01) (.yaw (Variables|Default|GetMax%20start%20%20rotation))))))
      (bind _alpha (Timeline|Timeline PlayFromStart)
        (:Update
          (Transformation|SetActorRotation (Math|Rotator|Lerp(Rotator) (Variables|Default|GetStarting%20Rotation_0) (Variables|Default|Getend%20rotation) _alpha true))
          (Utilities|FlowControl|DoOnce false :!label _label_2
            (:Completed
              (Default|CallBeginRotation (stale EventBeginPlay _outactors)))))
        (:Finished
          (Utilities|FlowControl|Sequence
            (:then_0
              (Default|CallEndRotation (stale EventBeginPlay _outactors))
              (goto _label Reset))
            (:then_1
              (goto _label_2 Reset))))))))

(event Custom|Reset%20rotation_Event
  (Transformation|SetActorRotation self "0, 0, 0" true))

(event EventBeginPlay
  (EventDispatchers|BindEventtoRotate (delegate Custom|Rotate_Event))
  (EventDispatchers|BindEventtoResetRotation (delegate Custom|Reset%20rotation_Event))
  (bind _outactors (Actor|GetAllActorsOfClass "/Game/GameDev/Alfie/lasers/BP_FinalSpawner.BP_FinalSpawner_C")))

(fn ConstructionScript)