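; BP_GrassMove is a grass actor that briefly changes colour to match the shell worn by an overlapping BP_Kyles_Character.
; On overlap, it compares the shell's first material against blue, green and red references and swaps the mesh to the matching material instance.
; After a short delay, it restores the default grass material.
; A one-shot timer shortly after BeginPlay runs the same check if the character reference is valid.
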(event Custom|Colour%20change
  (Utilities|IsValid (stale Collision|EventActorBeginOverlap _asbp_kyles_character)
    (:Is%20Valid
      (Utilities|FlowControl|Sequence
        (:then_0
          ;[1 1 1] SWITCHING COLOUR SHELLS
          (if (== (Rendering|Material|GetMaterial (Variables|/Game/Designers/Kyle/BP_Character/BP_Kyles_Character.BP_Kyles_Character_C|GetShell (stale Collision|EventActorBeginOverlap _asbp_kyles_character)) 0) "/Game/Progammers/Jack/Art/Materials/Mat_BlueDef.Mat_BlueDef")
            (Rendering|Material|SetMaterial (Variables|Default|GetStaticMesh) 0 "/Game/GameDev/MatthewG/Mechanics/Foliage/MI_BLUE.MI_BLUE")
            (Utilities|FlowControl|Delay 0.7)
            (Rendering|Material|SetMaterial (Variables|Default|GetStaticMesh) 0 "/Game/GameDev/MatthewG/Mechanics/Foliage/MI_Grass_Inst.MI_Grass_Inst")))
        (:then_1
          (if (== (Rendering|Material|GetMaterial (Variables|/Game/Designers/Kyle/BP_Character/BP_Kyles_Character.BP_Kyles_Character_C|GetShell (stale Collision|EventActorBeginOverlap _asbp_kyles_character)) 0) "/Game/Progammers/Jack/Art/Materials/Mat_GreenDef.Mat_GreenDef")
            (Rendering|Material|SetMaterial (Variables|Default|GetStaticMesh) 0 "/Game/GameDev/MatthewG/Mechanics/Foliage/MI_GREEN.MI_GREEN")
            (Utilities|FlowControl|Delay 0.7)
            (Rendering|Material|SetMaterial (Variables|Default|GetStaticMesh) 0 "/Game/GameDev/MatthewG/Mechanics/Foliage/MI_Grass_Inst.MI_Grass_Inst")))
        (:then_2
          (if (== (Rendering|Material|GetMaterial (Variables|/Game/Designers/Kyle/BP_Character/BP_Kyles_Character.BP_Kyles_Character_C|GetShell (stale Collision|EventActorBeginOverlap _asbp_kyles_character)) 0) "/Game/Progammers/Jack/Art/Materials/Mat_RedDef.Mat_RedDef")
            (Rendering|Material|SetMaterial (Variables|Default|GetStaticMesh) 0 "/Game/GameDev/MatthewG/Mechanics/Foliage/MI_RED.MI_RED")
            (Utilities|FlowControl|Delay 0.7)
            (Rendering|Material|SetMaterial (Variables|Default|GetStaticMesh) 0 "/Game/GameDev/MatthewG/Mechanics/Foliage/MI_Grass_Inst.MI_Grass_Inst")))))))

(event EventBeginPlay
  (Utilities|Time|SetTimerbyEvent (delegate Custom|Colour%20change) 0.1))

(event Collision|EventActorBeginOverlap
  (params (OtherActor :type Actor%20Object%20Reference))
  ;[1 1 1] CHECKING WHAT SHELL IS WORN
  (bind _asbp_kyles_character (Utilities|Casting|CastToBP_Kyles_Character OtherActor))
  (Utilities|FlowControl|Sequence
    (:then_0
      ;[1 1 1] SWITCHING COLOUR SHELLS
      (if (== (Rendering|Material|GetMaterial (Variables|/Game/Designers/Kyle/BP_Character/BP_Kyles_Character.BP_Kyles_Character_C|GetShell _asbp_kyles_character) 0) "/Game/Progammers/Jack/Art/Materials/Mat_BlueDef.Mat_BlueDef")
        (Rendering|Material|SetMaterial (Variables|Default|GetStaticMesh) 0 "/Game/GameDev/MatthewG/Mechanics/Foliage/MI_BLUE.MI_BLUE")
        (Utilities|FlowControl|Delay 0.7)
        (Rendering|Material|SetMaterial (Variables|Default|GetStaticMesh) 0 "/Game/GameDev/MatthewG/Mechanics/Foliage/MI_Grass_Inst.MI_Grass_Inst")))
    (:then_1
      (if (== (Rendering|Material|GetMaterial (Variables|/Game/Designers/Kyle/BP_Character/BP_Kyles_Character.BP_Kyles_Character_C|GetShell _asbp_kyles_character) 0) "/Game/Progammers/Jack/Art/Materials/Mat_GreenDef.Mat_GreenDef")
        (Rendering|Material|SetMaterial (Variables|Default|GetStaticMesh) 0 "/Game/GameDev/MatthewG/Mechanics/Foliage/MI_GREEN.MI_GREEN")
        (Utilities|FlowControl|Delay 0.7)
        (Rendering|Material|SetMaterial (Variables|Default|GetStaticMesh) 0 "/Game/GameDev/MatthewG/Mechanics/Foliage/MI_Grass_Inst.MI_Grass_Inst")))
    (:then_2
      (if (== (Rendering|Material|GetMaterial (Variables|/Game/Designers/Kyle/BP_Character/BP_Kyles_Character.BP_Kyles_Character_C|GetShell _asbp_kyles_character) 0) "/Game/Progammers/Jack/Art/Materials/Mat_RedDef.Mat_RedDef")
        (Rendering|Material|SetMaterial (Variables|Default|GetStaticMesh) 0 "/Game/GameDev/MatthewG/Mechanics/Foliage/MI_RED.MI_RED")
        (Utilities|FlowControl|Delay 0.7)
        (Rendering|Material|SetMaterial (Variables|Default|GetStaticMesh) 0 "/Game/GameDev/MatthewG/Mechanics/Foliage/MI_Grass_Inst.MI_Grass_Inst")))))

(fn ConstructionScript)