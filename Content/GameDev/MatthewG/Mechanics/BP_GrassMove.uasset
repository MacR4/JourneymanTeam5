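; BP_GrassMove is a grass actor that reacts to the player character overlapping it by briefly changing its material.
; On overlap with player 0's character, it swaps the static mesh to a second grass material instance, then restores the standard one after a short delay.
; A one-shot timer at BeginPlay also fires the ColourChange event, which feeds into the same player check.
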(event Custom|Colour%20change
  (if (== (Game|GetPlayerCharacter 0) (stale Collision|EventActorBeginOverlap OtherActor))
    (Rendering|Material|SetMaterial (Variables|Default|GetStaticMesh) 0 "/Game/GameDev/MatthewG/Mechanics/M_Grass_2_Inst.M_Grass_2_Inst")
    (Utilities|FlowControl|Delay 0.7)
    (Rendering|Material|SetMaterial (Variables|Default|GetStaticMesh) 0 "/Game/GameDev/MatthewG/Mechanics/MI_Grass_Inst.MI_Grass_Inst")))

(event EventBeginPlay
  (Utilities|Time|SetTimerbyEvent (delegate Custom|Colour%20change) 0.1))

(event Collision|EventActorBeginOverlap
  (params (OtherActor :type Actor%20Object%20Reference))
  (if (== (Game|GetPlayerCharacter 0) OtherActor)
    (Rendering|Material|SetMaterial (Variables|Default|GetStaticMesh) 0 "/Game/GameDev/MatthewG/Mechanics/M_Grass_2_Inst.M_Grass_2_Inst")
    (Utilities|FlowControl|Delay 0.7)
    (Rendering|Material|SetMaterial (Variables|Default|GetStaticMesh) 0 "/Game/GameDev/MatthewG/Mechanics/MI_Grass_Inst.MI_Grass_Inst")))

(fn ConstructionScript)