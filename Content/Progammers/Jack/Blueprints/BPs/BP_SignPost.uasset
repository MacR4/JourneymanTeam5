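; BP_SignPost is an interactable signpost that shows and hides a temporary sign widget.
; Its overlap collider sets IsLocal while BP_Kyles_Character is in range and stores the signpost in that character's LocalSignpostRef.
; InteractSignpost uses a FlipFlop to create or remove WBP_TempSignPost when in range, and only removes it when out of range.
; Leaving the collider neither removes the widget nor clears the character's reference.
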(event OnComponentBeginOverlap(IsLocalCollider)
  (params (OverlappedComponent :type Primitive%20Component%20Object%20Reference) (OtherActor :type Actor%20Object%20Reference) (OtherComp :type Primitive%20Component%20Object%20Reference) (OtherBodyIndex :type Integer) (bFromSweep :type Boolean) (SweepResult :type Hit%20Result%20Structure%20%28by%20ref%29))
  (bind _asbp_kyles_character (Utilities|Casting|CastToBP_Kyles_Character OtherActor))
  (Variables|/Game/Designers/Kyle/BP_Character/BP_Kyles_Character.BP_Kyles_Character_C|SetLocalSignpostRef _asbp_kyles_character self)
  (Variables|Default|SetIsLocal true)
  (Utilities|FlowControl|Delay 1.0))

(event OnComponentEndOverlap(IsLocalCollider)
  (params (OverlappedComponent :type Primitive%20Component%20Object%20Reference) (OtherActor :type Actor%20Object%20Reference) (OtherComp :type Primitive%20Component%20Object%20Reference) (OtherBodyIndex :type Integer))
  (Utilities|Casting|CastToBP_Kyles_Character OtherActor)
  (Variables|Default|SetIsLocal false)
  (Utilities|FlowControl|Delay 0.2))

(event Custom|InteractSignpost
  (if (Variables|Default|GetIsLocal)
    (Utilities|FlowControl|FlipFlop
      (:A
        (bind _returnvalue (UserInterface|CreateWidget "/Game/Progammers/Jack/Blueprints/Widgets/WBP_TempSignPost.WBP_TempSignPost_C" (Game|GetPlayerController 0)))
        (UserInterface|Viewport|AddtoViewport _returnvalue 0))
      (:B
        (Widget|RemovefromParent _returnvalue :!label _label)))
    (else
      (goto _label))))

(fn ConstructionScript)