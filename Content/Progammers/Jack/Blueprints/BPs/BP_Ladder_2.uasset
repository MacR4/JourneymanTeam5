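; Ladder actor that carries BP_Kyles_Character up a spline by setting its location from a Timeline-driven lerp over the spline length.
; Overlap triggers flag whether the player is near, lower or upper, and register the ladder and camera boom.
; MovePlayer, gated by a DoOnce, only climbs from the lower trigger; StopMoving halts the Timeline and resets the gate.
; Disconnected nodes hold unused camera-relative input movement experiments.
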(event OnComponentBeginOverlap(LowerTrigger)
  (params (OverlappedComponent :type Primitive%20Component%20Object%20Reference) (OtherActor :type Actor%20Object%20Reference) (OtherComp :type Primitive%20Component%20Object%20Reference) (OtherBodyIndex :type Integer) (bFromSweep :type Boolean) (SweepResult :type Hit%20Result%20Structure%20%28by%20ref%29))
  (Utilities|Casting|CastToBP_Kyles_Character OtherActor)
  (Variables|IsLocal|SetIsLocalLower true))

(event OnComponentEndOverlap(LowerTrigger)
  (params (OverlappedComponent :type Primitive%20Component%20Object%20Reference) (OtherActor :type Actor%20Object%20Reference) (OtherComp :type Primitive%20Component%20Object%20Reference) (OtherBodyIndex :type Integer))
  (Utilities|Casting|CastToBP_Kyles_Character OtherActor)
  (Variables|IsLocal|SetIsLocalLower false))

(event OnComponentBeginOverlap(PlayerLocalTrigger)
  (params (OverlappedComponent :type Primitive%20Component%20Object%20Reference) (OtherActor :type Actor%20Object%20Reference) (OtherComp :type Primitive%20Component%20Object%20Reference) (OtherBodyIndex :type Integer) (bFromSweep :type Boolean) (SweepResult :type Hit%20Result%20Structure%20%28by%20ref%29))
  (bind _asbp_kyles_character (Utilities|Casting|CastToBP_Kyles_Character OtherActor))
  (Variables|/Game/Designers/Kyle/BP_Character/BP_Kyles_Character.BP_Kyles_Character_C|SetLocalLadder2Ref _asbp_kyles_character self)
  (Variables|Default|SetCamera%20Boom (Variables|/Game/Designers/Kyle/BP_Character/BP_Kyles_Character.BP_Kyles_Character_C|GetCameraBoom _asbp_kyles_character))
  (Variables|IsLocal|SetIsLocalGeneral true))

(event OnComponentEndOverlap(PlayerLocalTrigger)
  (params (OverlappedComponent :type Primitive%20Component%20Object%20Reference) (OtherActor :type Actor%20Object%20Reference) (OtherComp :type Primitive%20Component%20Object%20Reference) (OtherBodyIndex :type Integer))
  (Utilities|Casting|CastToBP_Kyles_Character OtherActor)
  (Variables|IsLocal|SetIsLocalGeneral false))

(event OnComponentBeginOverlap(UpperTrigger)
  (params (OverlappedComponent :type Primitive%20Component%20Object%20Reference) (OtherActor :type Actor%20Object%20Reference) (OtherComp :type Primitive%20Component%20Object%20Reference) (OtherBodyIndex :type Integer) (bFromSweep :type Boolean) (SweepResult :type Hit%20Result%20Structure%20%28by%20ref%29))
  (Utilities|Casting|CastToBP_Kyles_Character OtherActor)
  (Variables|IsLocal|SetIsLocalUpper true))

(event OnComponentEndOverlap(UpperTrigger)
  (params (OverlappedComponent :type Primitive%20Component%20Object%20Reference) (OtherActor :type Actor%20Object%20Reference) (OtherComp :type Primitive%20Component%20Object%20Reference) (OtherBodyIndex :type Integer))
  (Utilities|Casting|CastToBP_Kyles_Character OtherActor)
  (Variables|IsLocal|SetIsLocalUpper false))

(event Custom|ResetDoOnce
  (bind _spline (Variables|Default|GetSpline))
  (Utilities|FlowControl|DoOnce false) ; enters at Reset
)

(event Custom|MovePlayer
  (bind _spline (Variables|Default|GetSpline))
  (Utilities|FlowControl|DoOnce false
    (:Completed
      (if (Variables|IsLocal|GetIsLocalLower)
        (bind _alpha (Timeline|Timeline PlayFromStart)
          (:Update
            (Transformation|SetActorLocation (Variables|Default|GetPlayer) (Spline|GetLocationatDistanceAlongSpline _spline (Math|Float|Lerp 0.0 (Spline|GetSplineLength _spline) _alpha) "World") false false)))))))

(event Custom|StopMoving
  (bind _spline (Variables|Default|GetSpline))
  (Utilities|FlowControl|Sequence
    (:then_0
      (bind _alpha (Timeline|Timeline Stop)
        (:Update
          (Transformation|SetActorLocation (Variables|Default|GetPlayer) (Spline|GetLocationatDistanceAlongSpline _spline (Math|Float|Lerp 0.0 (Spline|GetSplineLength _spline) _alpha) "World") false false))))
    (:then_1
      (CallFunction|ResetDoOnce))))

(event EventBeginPlay
  (bind _asbp_kyles_character (Utilities|Casting|CastToBP_Kyles_Character (Game|GetPlayerCharacter 0)))
  (Variables|Default|SetPlayer _asbp_kyles_character))

(fn ConstructionScript)