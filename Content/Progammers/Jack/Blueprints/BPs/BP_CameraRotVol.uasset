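; BP_CameraRotVol is a trigger volume that rotates the camera boom of BP_Kyles_Character when that character overlaps it.
; Begin overlap stores the boom's world rotation and plays the RotationLerp timeline, interpolating yaw toward TargetRotation while keeping pitch and roll.
; Each update passes that absolute interpolated rotation to AddWorldRotation, so it accumulates as a delta rather than setting the rotation.
; End overlap only casts, so nothing restores the camera.
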(event OnComponentBeginOverlap(CameraAdjustVol)
  (params (OverlappedComponent :type Primitive%20Component%20Object%20Reference) (OtherActor :type Actor%20Object%20Reference) (OtherComp :type Primitive%20Component%20Object%20Reference) (OtherBodyIndex :type Integer) (bFromSweep :type Boolean) (SweepResult :type Hit%20Result%20Structure%20%28by%20ref%29))
  (bind _asbp_kyles_character (Utilities|Casting|CastToBP_Kyles_Character OtherActor))
  (bind _output_get (Variables|Default|SetAs%20BP%20Kyles%20Character _asbp_kyles_character))
  (bind _output_get_2 (Variables|Default|SetCamera%20Boom (Variables|/Game/Designers/Kyle/BP_Character/BP_Kyles_Character.BP_Kyles_Character_C|GetCameraBoom _output_get)))
  (bind _output_get_3 (Variables|Default|SetDefaultRotation (Transformation|GetWorldRotation _output_get_2)))
  (bind _alpha_rot (Timeline|RotationLerp PlayFromStart)
    (:Update
      (Transformation|AddWorldRotation _output_get_2 (Math|Rotator|Lerp(Rotator) _output_get_3 (Math|Rotator|MakeRotator (.roll (Variables|Default|GetDefaultRotation)) (.pitch (Variables|Default|GetDefaultRotation)) (Variables|Default|GetTarget%20Rotation)) _alpha_rot) false true))))

(event OnComponentEndOverlap(CameraAdjustVol)
  (params (OverlappedComponent :type Primitive%20Component%20Object%20Reference) (OtherActor :type Actor%20Object%20Reference) (OtherComp :type Primitive%20Component%20Object%20Reference) (OtherBodyIndex :type Integer))
  (Utilities|Casting|CastToBP_Kyles_Character OtherActor))

(fn ConstructionScript)