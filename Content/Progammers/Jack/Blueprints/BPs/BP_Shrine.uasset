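; BP_Shrine is an interactable shrine that plays a day-night cycle by rotating the level's directional light.
; A trigger overlap marks the player as local, hands over a shrine reference and updates the object info.
; Interaction runs through a resettable DoOnce and, if local, starts a timeline that lerps the light's pitch.
; Respawn, stat restore and interaction-count logic is present but disconnected.
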(event OnComponentBeginOverlap(CheckpointTrigger)
  (params (OverlappedComponent :type Primitive%20Component%20Object%20Reference) (OtherActor :type Actor%20Object%20Reference) (OtherComp :type Primitive%20Component%20Object%20Reference) (OtherBodyIndex :type Integer) (bFromSweep :type Boolean) (SweepResult :type Hit%20Result%20Structure%20%28by%20ref%29))
  ;[0 0.1319 1] Is Local Checks
  (bind _asbp_kyles_character (Utilities|Casting|CastToBP_Kyles_Character OtherActor))
  (bind _output_get (Variables|Default|SetPlayer _asbp_kyles_character))
  (Variables|/Game/Designers/Kyle/BP_Character/BP_Kyles_Character.BP_Kyles_Character_C|SetLocalShrineRef _output_get self)
  (Variables|Default|SetIsLocal true)
  ;[0.3864 0.2122 0.3864] Update Object Info
  (CallFunction|UpdateOBJInfo (Variables|Default|GetObjectInfoText) true (Variables|Default|GetMax%20Num%20Interactions) (Variables|Default|GetMapKey)))

(event OnComponentEndOverlap(CheckpointTrigger)
  (params (OverlappedComponent :type Primitive%20Component%20Object%20Reference) (OtherActor :type Actor%20Object%20Reference) (OtherComp :type Primitive%20Component%20Object%20Reference) (OtherBodyIndex :type Integer))
  ;[0 0.1319 1] Is Local Checks
  (Utilities|Casting|CastToBP_Kyles_Character OtherActor)
  (Variables|Default|SetIsLocal false))

(event Custom|Interact%20With%20Shrine
  (bind _directionallight (Variables|Default|GetDirectionalLight))
  (bind _returnvalue (Transformation|GetActorRotation _directionallight))
  (bind (_roll _pitch _yaw) (Math|Rotator|BreakRotator _returnvalue))
  ;[1 0.8673 0.227] Interaction
  (Utilities|FlowControl|DoOnce false
    (:Completed
      (if (Variables|Default|GetIsLocal)
        (bind _alpha (Timeline|Day/Night%20Cycle PlayFromStart)
          (:Update
            (Transformation|SetActorRotation _directionallight (Math|Rotator|Lerp(Rotator) _returnvalue (Math|Rotator|MakeRotator _roll (+ _pitch 3.6e+02) _yaw) _alpha))))))))

(event Custom|ResetDoOnce
  (bind _directionallight (Variables|Default|GetDirectionalLight))
  (bind _returnvalue (Transformation|GetActorRotation _directionallight))
  (bind (_roll _pitch _yaw) (Math|Rotator|BreakRotator _returnvalue))
  ;[1 0.8673 0.227] Interaction
  (Utilities|FlowControl|DoOnce false) ; enters at Reset
)

(event EventBeginPlay
  (bind _returnvalue (Actor|GetActorOfClass "/Script/Engine.DirectionalLight"))
  (Variables|Default|SetDirectionalLight _returnvalue))

(fn ConstructionScript)