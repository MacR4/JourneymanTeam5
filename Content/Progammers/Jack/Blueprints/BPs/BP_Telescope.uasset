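; BP_Telescope is an interactable telescope that moves the player's camera to a viewing point and back.
; Overlapping TelescopeTrigger caches the BP_Kyles_Character and its CameraBoom.
; UniversalInteraction alternates between locking movement while a timeline lerps the boom to LocationSphere, and restoring movement while reversing that timeline.
; A DoOnce blocks further interactions until the timeline finishes.
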(event OnComponentBeginOverlap(TelescopeTrigger)
  (params (OverlappedComponent :type Primitive%20Component%20Object%20Reference) (OtherActor :type Actor%20Object%20Reference) (OtherComp :type Primitive%20Component%20Object%20Reference) (OtherBodyIndex :type Integer) (bFromSweep :type Boolean) (SweepResult :type Hit%20Result%20Structure%20%28by%20ref%29))
  (bind _asbp_kyles_character (Utilities|Casting|CastToBP_Kyles_Character OtherActor))
  (bind _output_get (Variables|Default|SetPlayer _asbp_kyles_character))
  (Variables|Default|SetCamera%20Boom (Variables|/Game/Designers/Kyle/BP_Character/BP_Kyles_Character.BP_Kyles_Character_C|GetCameraBoom _output_get)))

(event Custom|Reset%20Do%20Once
  (bind _player (Variables|Default|GetPlayer))
  (Utilities|FlowControl|DoOnce false) ; enters at Reset
)

(event EventUniversalInteraction
  (bind _player (Variables|Default|GetPlayer))
  (Utilities|FlowControl|DoOnce false
    (:Completed
      (Utilities|FlowControl|FlipFlop
        (:A
          (Variables|/Game/Designers/Kyle/BP_Character/BP_Kyles_Character.BP_Kyles_Character_C|SetIsMoveable _player false)
          (bind _output_get (Variables|Default|SetCameraStartLoc (Transformation|GetWorldLocation (Variables|Default|GetCamera%20Boom))))
          (bind _alpha (Timeline|CameraLocAlpha PlayFromStart)
            (:Update
              (Transformation|SetWorldLocation (Variables|Default|GetCamera%20Boom) (Math|Vector|Lerp(Vector) _output_get (Transformation|GetWorldLocation (Variables|Default|GetLocationSphere)) _alpha) false false))
            (:Finished
              (CallFunction|ResetDoOnce))))
        (:B
          (Variables|/Game/Designers/Kyle/BP_Character/BP_Kyles_Character.BP_Kyles_Character_C|SetIsMoveable _player true)
          (Timeline|CameraLocAlpha ReverseFromEnd))))))

(fn ConstructionScript)