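; Interactable lever that activates a linked laser spawner.
; Its UniversalInteraction event calls ActivateEvent on the BPLaserspawner reference.
; The IsLocalTrigger overlap sets IsLocal and updates the object info with text, key and interaction limit, then clears IsLocal on exit.
; An IsLocal-gated path to the same activation exists but is never run.
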(event OnComponentBeginOverlap(IsLocalTrigger)
  (params (OverlappedComponent :type Primitive%20Component%20Object%20Reference) (OtherActor :type Actor%20Object%20Reference) (OtherComp :type Primitive%20Component%20Object%20Reference) (OtherBodyIndex :type Integer) (bFromSweep :type Boolean) (SweepResult :type Hit%20Result%20Structure%20%28by%20ref%29))
  (Variables|Default|SetIsLocal true)
  (CallFunction|UpdateOBJInfo (Variables|Default|GetObj%20Info%20Text) (Variables|Default|GetMax%20Num%20Interactions) true (Utilities|String|EnumtoString (Variables|Default|GetKey))))

(event OnComponentEndOverlap(IsLocalTrigger)
  (params (OverlappedComponent :type Primitive%20Component%20Object%20Reference) (OtherActor :type Actor%20Object%20Reference) (OtherComp :type Primitive%20Component%20Object%20Reference) (OtherBodyIndex :type Integer))
  (Variables|Default|SetIsLocal false))

(event EventUniversalInteraction
  (Default|ActivateEvent (Variables|Default|GetBP_laserspawner)))

(event Input|KeyboardEvents|SpaceBar
  (params (Key :type Key%20Structure :default "None")))

(fn ConstructionScript
  (|CallParentFunction))