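; BP_DamagingVolume is a volume that deals repeated damage to a BP_Kyles_Character inside it.
; Beginning overlap with DamageVol stores the character, sets the IsLocal flag and starts the damage loop.
; DealDamage applies DamageAmount, waits DamageFrequency, then calls itself while PlayerHealth is above zero.
; Any end overlap clears IsLocal without checking the actor, so the next loop pass deals no damage and stops.
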(event OnComponentBeginOverlap(DamageVol)
  (params (OverlappedComponent :type Primitive%20Component%20Object%20Reference) (OtherActor :type Actor%20Object%20Reference) (OtherComp :type Primitive%20Component%20Object%20Reference) (OtherBodyIndex :type Integer) (bFromSweep :type Boolean) (SweepResult :type Hit%20Result%20Structure%20%28by%20ref%29))
  (bind _asbp_kyles_character (Utilities|Casting|CastToBP_Kyles_Character OtherActor))
  (bind _output_get (Variables|Default|SetIsLocal true))
  (if _output_get
    (Default|TakeDamage _asbp_kyles_character (Variables|Default|GetDamageAmount))
    (Utilities|FlowControl|Delay (Variables|Default|GetDamageFrequency))
    (if (> (Variables|/Game/Designers/Kyle/BP_Character/BP_Kyles_Character.BP_Kyles_Character_C|GetPlayer%20Health _asbp_kyles_character) 0.0)
      (CallFunction|DealDamage))))

(event OnComponentEndOverlap(DamageVol)
  (params (OverlappedComponent :type Primitive%20Component%20Object%20Reference) (OtherActor :type Actor%20Object%20Reference) (OtherComp :type Primitive%20Component%20Object%20Reference) (OtherBodyIndex :type Integer))
  (Variables|Default|SetIsLocal false))

(event Custom|Deal%20Damage
  (if (stale OnComponentBeginOverlap(DamageVol) _output_get)
    (Default|TakeDamage (stale OnComponentBeginOverlap(DamageVol) _asbp_kyles_character) (Variables|Default|GetDamageAmount))
    (Utilities|FlowControl|Delay (Variables|Default|GetDamageFrequency))
    (if (> (Variables|/Game/Designers/Kyle/BP_Character/BP_Kyles_Character.BP_Kyles_Character_C|GetPlayer%20Health (stale OnComponentBeginOverlap(DamageVol) _asbp_kyles_character)) 0.0)
      (CallFunction|DealDamage))))

(fn ConstructionScript)