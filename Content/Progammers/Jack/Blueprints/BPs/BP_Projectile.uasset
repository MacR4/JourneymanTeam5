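; BP_Projectile is a projectile actor that homes in on a jar or wall referenced by Kyle's player character, which it caches on BeginPlay.
; BreakJar and BreakWall each validate the player's local target reference, then run their own timeline to lerp the projectile from its current location toward that target, printing debug text.
; When the timeline finishes, the projectile destroys itself and calls ResetDoOnce on the target.
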(event Custom|BreakJar
  (bind _player (Variables|Default|GetPlayer))
  (bind _localjarref (Variables|/Game/Designers/Kyle/BP_Character/BP_Kyles_Character.BP_Kyles_Character_C|GetLocalJarRef _player))
  (Utilities|IsValid _localjarref
    (:Is%20Valid
      (bind _alpha (Timeline|ProjectileLerp PlayFromStart)
        (:Update
          (Transformation|SetActorLocation (Math|Vector|Lerp(Vector) (Transformation|GetActorLocation self) (Transformation|GetActorLocation _localjarref) _alpha) false false)
          (Development|PrintString "Breaking Jars"))
        (:Finished
          (Actor|DestroyActor)
          (Default|ResetDoOnce _localjarref))))))

(event Custom|BreakWall
  (bind _player (Variables|Default|GetPlayer))
  (bind _localwallref (Variables|/Game/Designers/Kyle/BP_Character/BP_Kyles_Character.BP_Kyles_Character_C|GetLocalWallRef _player))
  (Utilities|IsValid _localwallref
    (:Is%20Valid
      (bind _alpha (Timeline|Timeline PlayFromStart)
        (:Update
          (Transformation|SetActorLocation (Math|Vector|Lerp(Vector) (Transformation|GetActorLocation self) (Transformation|GetActorLocation _localwallref) _alpha) false false)
          (Development|PrintString "Breaking Walls"))
        (:Finished
          (Actor|DestroyActor)
          (Default|ResetDoOnce _localwallref))))))

(event EventBeginPlay
  (bind _asbp_kyles_character (Utilities|Casting|CastToBP_Kyles_Character (Game|GetPlayerCharacter 0)))
  (Variables|Default|SetPlayer _asbp_kyles_character))

(fn ConstructionScript)