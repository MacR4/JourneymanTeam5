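; BP_Ladder is a climbable ladder that moves BP_Kyles_Character along a spline, up or down.
; Colliders at each end record the player and direction; the up collider also registers the ladder on the character and updates objective text.
; A DoOnce-gated PlayerUseLadder uses timelines to lerp the player onto the nearest spline end, then along it.
; CancelLadder stops only the approach timelines when velocity points away from the ladder.
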(event OnComponentBeginOverlap(LadderColliderUp)
  (params (OverlappedComponent :type Primitive%20Component%20Object%20Reference) (OtherActor :type Actor%20Object%20Reference) (OtherComp :type Primitive%20Component%20Object%20Reference) (OtherBodyIndex :type Integer) (bFromSweep :type Boolean) (SweepResult :type Hit%20Result%20Structure%20%28by%20ref%29))
  ;[0.3183 1 0.3354] Collision Logic Up
  (bind _asbp_kyles_character (Utilities|Casting|CastToBP_Kyles_Character OtherActor))
  (Variables|Default|SetPlayer _asbp_kyles_character)
  (Variables|Default|SetIsLocalUp true)
  (Variables|/Game/Designers/Kyle/BP_Character/BP_Kyles_Character.BP_Kyles_Character_C|SetLocalLadderRef _asbp_kyles_character self)
  (if (< (Variables|/Game/Designers/Kyle/BP_Character/BP_Kyles_Character.BP_Kyles_Character_C|GetNumLadderInteract _asbp_kyles_character) 3)
    (CallFunction|UpdateOBJInfo (Variables|Default|GetObjectInfoText) (Variables|Default|GetNum%20Interactions) (Variables|Default|GetMax%20Num%20Interactions) false)))

(event OnComponentBeginOverlap(LadderColliderDown)
  (params (OverlappedComponent :type Primitive%20Component%20Object%20Reference) (OtherActor :type Actor%20Object%20Reference) (OtherComp :type Primitive%20Component%20Object%20Reference) (OtherBodyIndex :type Integer) (bFromSweep :type Boolean) (SweepResult :type Hit%20Result%20Structure%20%28by%20ref%29))
  ;[1 0.3194 0.2975] Collision Logic Down
  (bind _asbp_kyles_character (Utilities|Casting|CastToBP_Kyles_Character OtherActor))
  (Variables|Default|SetPlayer _asbp_kyles_character)
  (Variables|Default|SetIsLocalDown true))

(event OnComponentEndOverlap(LadderColliderUp)
  (params (OverlappedComponent :type Primitive%20Component%20Object%20Reference) (OtherActor :type Actor%20Object%20Reference) (OtherComp :type Primitive%20Component%20Object%20Reference) (OtherBodyIndex :type Integer))
  ;[0.3183 1 0.3354] Collision Logic Up
  (Variables|Default|SetIsLocalUp false))

(event OnComponentEndOverlap(LadderColliderDown)
  (params (OverlappedComponent :type Primitive%20Component%20Object%20Reference) (OtherActor :type Actor%20Object%20Reference) (OtherComp :type Primitive%20Component%20Object%20Reference) (OtherBodyIndex :type Integer))
  ;[1 0.3194 0.2975] Collision Logic Down
  (Variables|Default|SetIsLocalDown false))

(event Custom|ResetDoOnce
  (bind _player (Variables|Default|GetPlayer))
  (bind _player_2 (Variables|Default|GetPlayer))
  (bind _player_3 (Variables|Default|GetPlayer))
  (bind _playerpathway (Variables|Default|GetPlayerPathway))
  (bind _returnvalue (Spline|GetSplineLength _playerpathway))
  ;[1 1 1] Interact Input
  (Utilities|FlowControl|DoOnce false) ; enters at Reset
)

(event Custom|CancelClimbing
  (bind _player (Variables|Default|GetPlayer))
  (bind _player_2 (Variables|Default|GetPlayer))
  (bind _playerpathway (Variables|Default|GetPlayerPathway))
  (bind _returnvalue (Spline|GetSplineLength _playerpathway))
  (Development|PrintString "Cancelling Climbing")
  (Utilities|FlowControl|Sequence
    (:then_0
      ;[0.3216 1 0.2455] Move Player Up
      (bind _alpha (Timeline|Move%20To%20Spline%20Up Stop)
        (:Update
          (Transformation|SetActorLocation _player (Math|Vector|Lerp(Vector) (Transformation|GetActorLocation _player) (Spline|GetLocationatDistanceAlongSpline _playerpathway 0.0 "World") _alpha) false false))
        (:Finished
          (bind _alpha_2 (Timeline|Move%20Up%20Spline PlayFromStart)
            (:Update
              (Transformation|SetActorLocation (stale OnComponentBeginOverlap(LadderColliderUp) _asbp_kyles_character) (Spline|GetLocationatDistanceAlongSpline _playerpathway (Math|Float|Lerp 0.0 _returnvalue _alpha_2) "World") false false))
            (:Finished
              (CallFunction|ResetDoOnce :!label _label))))))
    (:then_1
      ;[1 0.1195 0.1932] Move Player Down
      (bind _alpha_3 (Timeline|Move%20To%20Spline Stop)
        (:Update
          (Transformation|SetActorLocation _player_2 (Math|Vector|Lerp(Vector) (Transformation|GetActorLocation _player_2) (Spline|GetLocationatDistanceAlongSpline _playerpathway _returnvalue "World") _alpha_3) false false))
        (:Finished
          (bind _alpha_4 (Timeline|Move%20Down%20Spline PlayFromStart)
            (:Update
              (Transformation|SetActorLocation (stale OnComponentBeginOverlap(LadderColliderDown) _asbp_kyles_character) (Spline|GetLocationatDistanceAlongSpline _playerpathway (Math|Float|Lerp _returnvalue 0.0 _alpha_4) "World") false false))
            (:Finished
              (goto _label))))))))

(event Custom|CancelLadder
  (bind _player (Variables|Default|GetPlayer))
  (if (>= (Math|Vector|DotProduct (Math|Vector|Normalize (- (Transformation|GetActorLocation _player) (Transformation|GetActorLocation self))) (Math|Vector|Normalize (Transformation|GetVelocity _player))) 0.8)
    (Development|PrintString "Cancelled climbing")
    (CallFunction|CancelClimbing)))

(event Custom|PlayerUseLadder
  (bind _player (Variables|Default|GetPlayer))
  (bind _player_2 (Variables|Default|GetPlayer))
  (bind _player_3 (Variables|Default|GetPlayer))
  (bind _playerpathway (Variables|Default|GetPlayerPathway))
  (bind _returnvalue (Spline|GetSplineLength _playerpathway))
  ;[1 1 1] Interact Input
  (Utilities|FlowControl|DoOnce false
    (:Completed
      (Utilities|FlowControl|Sequence
        (:then_0
          ;[0.3216 1 0.2455] Move Player Up
          (Variables|/Game/Designers/Kyle/BP_Character/BP_Kyles_Character.BP_Kyles_Character_C|SetNumLadderInteract _player (+ (Variables|/Game/Designers/Kyle/BP_Character/BP_Kyles_Character.BP_Kyles_Character_C|GetNumLadderInteract _player) 1))
          (if (Variables|Default|GetIsLocalUp)
            (bind _alpha (Timeline|Move%20To%20Spline%20Up PlayFromStart)
              (:Update
                (Transformation|SetActorLocation _player_2 (Math|Vector|Lerp(Vector) (Transformation|GetActorLocation _player_2) (Spline|GetLocationatDistanceAlongSpline _playerpathway 0.0 "World") _alpha) false false))
              (:Finished
                (bind _alpha_2 (Timeline|Move%20Up%20Spline PlayFromStart)
                  (:Update
                    (Transformation|SetActorLocation (stale OnComponentBeginOverlap(LadderColliderUp) _asbp_kyles_character) (Spline|GetLocationatDistanceAlongSpline _playerpathway (Math|Float|Lerp 0.0 _returnvalue _alpha_2) "World") false false))
                  (:Finished
                    (CallFunction|ResetDoOnce :!label _label)))))))
        (:then_1
          ;[1 0.1195 0.1932] Move Player Down
          (if (Variables|Default|GetIsLocalDown)
            (bind _alpha_3 (Timeline|Move%20To%20Spline PlayFromStart)
              (:Update
                (Transformation|SetActorLocation _player_3 (Math|Vector|Lerp(Vector) (Transformation|GetActorLocation _player_3) (Spline|GetLocationatDistanceAlongSpline _playerpathway _returnvalue "World") _alpha_3) false false))
              (:Finished
                (bind _alpha_4 (Timeline|Move%20Down%20Spline PlayFromStart)
                  (:Update
                    (Transformation|SetActorLocation (stale OnComponentBeginOverlap(LadderColliderDown) _asbp_kyles_character) (Spline|GetLocationatDistanceAlongSpline _playerpathway (Math|Float|Lerp _returnvalue 0.0 _alpha_4) "World") false false))
                  (:Finished
                    (goto _label)))))))))))

(fn ConstructionScript)