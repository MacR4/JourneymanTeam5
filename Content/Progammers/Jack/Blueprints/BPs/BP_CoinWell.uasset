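; BP_CoinWell is a coin well that accumulates tossed coins toward a maximum.
; TossCoin adds coins through AddCoins, which reports true only when the total exactly equals MaxCoins; the event then prints "Added Card Slot" without granting anything itself.
; A separate IsLocalCollider overlap sets IsLocal while a BP_Kyles_Character is inside, though the flag is not read in these graphs.
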(event OnComponentBeginOverlap(IsLocalCollider)
  (params (OverlappedComponent :type Primitive%20Component%20Object%20Reference) (OtherActor :type Actor%20Object%20Reference) (OtherComp :type Primitive%20Component%20Object%20Reference) (OtherBodyIndex :type Integer) (bFromSweep :type Boolean) (SweepResult :type Hit%20Result%20Structure%20%28by%20ref%29))
  (Utilities|Casting|CastToBP_Kyles_Character OtherActor)
  (Variables|Default|SetIsLocal true))

(event OnComponentEndOverlap(IsLocalCollider)
  (params (OverlappedComponent :type Primitive%20Component%20Object%20Reference) (OtherActor :type Actor%20Object%20Reference) (OtherComp :type Primitive%20Component%20Object%20Reference) (OtherBodyIndex :type Integer))
  (Utilities|Casting|CastToBP_Kyles_Character OtherActor)
  (Variables|Default|SetIsLocal false))

(event Custom|Toss%20Coin
  (params (CoinsToAdd :type Integer))
  (bind _ismax (CallFunction|AddCoins CoinsToAdd))
  (if _ismax
    (Development|PrintString "Added Card Slot")))

(fn ConstructionScript)

(fn AddCoins
  (params (CoinsToAdd :type Integer))
  (bind _output_get (Variables|Default|SetCurrentCoins (+ (Variables|Default|GetCurrentCoins) CoinsToAdd)))
  (return (== _output_get (Variables|Default|GetMaxCoins))))