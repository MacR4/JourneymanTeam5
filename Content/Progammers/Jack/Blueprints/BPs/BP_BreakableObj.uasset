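; Breakable object actor, such as a jar, that shatters through a Chaos geometry collection and then cleans itself up.
; A sphere overlap marks it local, registers it on the Kyles character and updates object interaction info.
; BreakJar, gated on that local flag, briefly enables the Cube's collision.
; The Chaos break event later disables the collection's collision and destroys the actor after delays.
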(event OnComponentBeginOverlap(Sphere)
  (params (OverlappedComponent :type Primitive%20Component%20Object%20Reference) (OtherActor :type Actor%20Object%20Reference) (OtherComp :type Primitive%20Component%20Object%20Reference) (OtherBodyIndex :type Integer) (bFromSweep :type Boolean) (SweepResult :type Hit%20Result%20Structure%20%28by%20ref%29))
  ;[0.4542 0.8796 1] Is Local checks
  (bind _asbp_kyles_character (Utilities|Casting|CastToBP_Kyles_Character OtherActor))
  (Variables|Default|SetAs%20BP%20Kyles%20Character _asbp_kyles_character)
  (Variables|Default|SetIsLocal true)
  (Variables|/Game/Designers/Kyle/BP_Character/BP_Kyles_Character.BP_Kyles_Character_C|SetLocalJarRef _asbp_kyles_character self)
  (CallFunction|UpdateOBJInfo (Variables|Default|GetObj%20Info%20Text) (Variables|Default|GetMax%20Num%20Interactions) true (Utilities|String|EnumtoString (Variables|Default|GetKey))))

(event OnChaosBreakEvent(Object_GC)
  (params (BreakEvent :type Chaos%20Break%20Event%20Structure%20%28by%20ref%29))
  ;[0.4937 1 0.6909] Object broken
  (Utilities|FlowControl|Delay (Variables|Default|GetCollision%20Delay))
  (Collision|SetCollisionEnabled (Variables|Default|GetObject_GC) "NoCollision")
  (Utilities|FlowControl|Delay 1.5)
  (Actor|DestroyActor))

(event OnComponentEndOverlap(Sphere)
  (params (OverlappedComponent :type Primitive%20Component%20Object%20Reference) (OtherActor :type Actor%20Object%20Reference) (OtherComp :type Primitive%20Component%20Object%20Reference) (OtherBodyIndex :type Integer))
  ;[0.4542 0.8796 1] Is Local checks
  (Utilities|Casting|CastToBP_Kyles_Character OtherActor)
  (Variables|Default|SetIsLocal false))

(event Custom|BreakJar
  (bind _cube (Variables|Default|GetCube))
  ;[0.8021 0.12 1] Make Object break
  (if (Variables|Default|GetIsLocal)
    (Collision|SetCollisionEnabled _cube "QueryAndPhysics")
    (Utilities|FlowControl|Delay 0.2)
    (Collision|SetCollisionEnabled _cube "NoCollision")))

(fn ConstructionScript)