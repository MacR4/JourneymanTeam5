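; BP_Lever_RotatorParent is an interactable lever that triggers rotation on a referenced rotator object.
; Overlapping its IsLocalTrigger with BP_Kyles_Character stores that player, sets the local flag and updates object info with the key and interaction limit; leaving clears the flag.
; UniversalInteraction calls CallRotate on the rotator, then records the interaction for the player through AddToInteractions.
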(event OnComponentBeginOverlap(IsLocalTrigger)
  (params (OverlappedComponent :type Primitive%20Component%20Object%20Reference) (OtherActor :type Actor%20Object%20Reference) (OtherComp :type Primitive%20Component%20Object%20Reference) (OtherBodyIndex :type Integer) (bFromSweep :type Boolean) (SweepResult :type Hit%20Result%20Structure%20%28by%20ref%29))
  (bind _key (Variables|Default|GetKey))
  (bind _returnvalue (Utilities|String|EnumtoString _key))
  (bind _asbp_kyles_character (Utilities|Casting|CastToBP_Kyles_Character OtherActor))
  (bind _output_get (Variables|Default|SetPlayer _asbp_kyles_character))
  (Variables|Default|SetIsLocal true)
  (bind _output_get_2 (Variables|Default|SetKeyString _returnvalue))
  (CallFunction|UpdateOBJInfo (Variables|Default|GetObj%20Info%20Text) true (Variables|Default|GetMax%20Num%20Interactions) _returnvalue))

(event OnComponentEndOverlap(IsLocalTrigger)
  (params (OverlappedComponent :type Primitive%20Component%20Object%20Reference) (OtherActor :type Actor%20Object%20Reference) (OtherComp :type Primitive%20Component%20Object%20Reference) (OtherBodyIndex :type Integer))
  (Utilities|Casting|CastToBP_Kyles_Character OtherActor)
  (Variables|Default|SetIsLocal false))

(event EventUniversalInteraction
  (Default|CallRotate (Variables|Default|GetBP%20Rotator%20Parent))
  (CallFunction|AddtoInteractions 0 (stale OnComponentBeginOverlap(IsLocalTrigger) _output_get_2) (stale OnComponentBeginOverlap(IsLocalTrigger) _output_get)))

(fn ConstructionScript
  (|CallParentFunction))