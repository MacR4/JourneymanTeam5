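; Torch actor that fakes a flickering fire with layered flame components and two spotlights.
; Tick, throttled by a short Delay, randomly yaws the inner, middle and outer flames and the first spotlight.
; It also randomizes both light intensities within set ranges, offsetting the second dimmer, and stores their current colours.
; A ColourLerp timeline for blending toward random palette colours exists but is never triggered.
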(event EventTick
  (params (DeltaSeconds :type Float%20%28single-precision%29))
  (bind _randomintensitymin_light (Variables|Default|GetRandomIntensityMin_Light))
  (bind _randomintensitymax_light (Variables|Default|GetRandomIntensityMax_Light))
  (bind _randomrotmin_flames (Variables|Default|GetRandomRotMin_Flames))
  (bind _randomrotmax_flames (Variables|Default|GetRandomRotMax_Flames))
  (bind _returnvalue (Math|Random|RandomFloatinRange _randomintensitymin_light _randomintensitymax_light))
  ;[1 0.5609 0.1562] Rotate Flames
  (Utilities|FlowControl|Delay 0.05)
  (Utilities|FlowControl|Sequence
    (:then_0
      (Transformation|AddWorldRotation (Variables|Default|GetFireInner) (Math|Rotator|MakeRotator 0.0 0.0 (Math|Random|RandomFloatinRange _randomrotmin_flames _randomrotmax_flames)) false false)
      ;[1 0.9807 0.3265] Rotate Light Source
      (Transformation|AddWorldRotation (Variables|Default|GetSpotLight1) (Math|Rotator|MakeRotator 0.0 0.0 (Math|Random|RandomFloatinRange (Variables|Default|GetRandomRotMin_Light) (Variables|Default|GetRandomRotMax_Light))) false false)
      ;[1 0.0625 0.0625] Set Intensity
      (Rendering|Components|Light|SetIntensity (Variables|Default|GetSpotLight1) _returnvalue)
      (Rendering|Components|Light|SetIntensity (Variables|Default|GetSpotLight2) (- _returnvalue 2e+03))
      (bind _output_get (Variables|Default|SetCurrentColourSpot1 (Rendering|Components|Light|GetLightColor (Variables|Default|GetSpotLight1))))
      (bind _output_get_2 (Variables|Default|SetCurrentColourSpot2 (Rendering|Components|Light|GetLightColor (Variables|Default|GetSpotLight2)))))
    (:then_1
      (Transformation|AddWorldRotation (Variables|Default|GetFireMid) (Math|Rotator|MakeRotator 0.0 0.0 (Math|Random|RandomFloatinRange _randomrotmin_flames _randomrotmax_flames)) false false))
    (:then_2
      (Transformation|AddWorldRotation (Variables|Default|GetFireOuter) (Math|Rotator|MakeRotator 0.0 0.0 (Math|Random|RandomFloatinRange _randomrotmin_flames _randomrotmax_flames)) false false))))

(fn ConstructionScript)