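; Test actor that procedurally duplicates static meshes at fixed spacing from configurable X and Y step counts.
; The construction script's outer loop adds meshes along X, and a nested loop adds a row along Y on each pass.
; Inner meshes set only a Y offset, so each pass repeats the same positions instead of forming a grid.
; The event graph holds only disabled placeholder events.
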(event EventBeginPlay)

(event Collision|EventActorBeginOverlap
  (params (OtherActor :type Actor%20Object%20Reference)))

(event EventTick
  (params (DeltaSeconds :type Float%20%28single-precision%29)))

(fn ConstructionScript
  (Variables|Default|SetNumberOfStepsY (Variables|Default|GetNumberOfStepsY_Default))
  (for _index (range 0 (- (Variables|Default|GetNumberOfStepsX) 1))
    (AddComponent|AddStaticMeshComponent false (Math|Transform|MakeTransform (Math|Vector|MakeVector (Math|Conversions|ToFloat(Integer) (* _index 70)) 0.0 0.0) "0, 0, 0" "1.000000,1.000000,1.000000"))
    (for _index_2 (range 0 (- (Variables|Default|GetNumberOfStepsY) 1))
      (AddComponent|AddStaticMeshComponent false (Math|Transform|MakeTransform (Math|Vector|MakeVector 0.0 (Math|Conversions|ToFloat(Integer) (* _index_2 70)) 0.0) "0, 0, 0" "1.000000,1.000000,1.000000")))
    (Variables|Default|SetNumberOfStepsY (Variables|Default|GetNumberOfStepsY_Default))))