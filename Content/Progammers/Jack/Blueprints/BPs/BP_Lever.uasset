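; BP_Lever is a lever that opens its linked door when interacted with while a player character is nearby.
; Entering the IsLocalTrigger volume stores the lever as LocalLeverRef on BP_Kyles_Character and sets IsLocal; leaving clears only the flag.
; InteractLever calls OpenDoor on LinkedDoor only while IsLocal is true.
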(event OnComponentBeginOverlap(IsLocalTrigger)
  (params (OverlappedComponent :type Primitive%20Component%20Object%20Reference) (OtherActor :type Actor%20Object%20Reference) (OtherComp :type Primitive%20Component%20Object%20Reference) (OtherBodyIndex :type Integer) (bFromSweep :type Boolean) (SweepResult :type Hit%20Result%20Structure%20%28by%20ref%29))
  (bind _asbp_kyles_character (Utilities|Casting|CastToBP_Kyles_Character OtherActor))
  (Variables|/Game/Designers/Kyle/BP_Character/BP_Kyles_Character.BP_Kyles_Character_C|SetLocalLeverRef _asbp_kyles_character self)
  (Variables|Default|SetIsLocal true))

(event OnComponentEndOverlap(IsLocalTrigger)
  (params (OverlappedComponent :type Primitive%20Component%20Object%20Reference) (OtherActor :type Actor%20Object%20Reference) (OtherComp :type Primitive%20Component%20Object%20Reference) (OtherBodyIndex :type Integer))
  (Utilities|Casting|CastToBP_Kyles_Character OtherActor)
  (Variables|Default|SetIsLocal false))

(event Custom|InteractLever
  (if (Variables|Default|GetIsLocal)
    (Default|OpenDoor (Variables|Default|GetLinkedDoor))))

(fn ConstructionScript)