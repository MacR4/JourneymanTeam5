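; BP_Chest is an interactable chest that gives a shell to a BP_Kyles_Character within range.
; ChestCollider overlaps set the IsLocal proximity flag and write the chest to the character's LocalChestRef, on exit as well as entry.
; InteractWithChest checks IsLocal, then uses EnumItemOptions to add a blue, red or green shell to the character cached on overlap.
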(event OnComponentBeginOverlap(ChestCollider)
  (params (OverlappedComponent :type Primitive%20Component%20Object%20Reference) (OtherActor :type Actor%20Object%20Reference) (OtherComp :type Primitive%20Component%20Object%20Reference) (OtherBodyIndex :type Integer) (bFromSweep :type Boolean) (SweepResult :type Hit%20Result%20Structure%20%28by%20ref%29))
  (bind _asbp_kyles_character (Utilities|Casting|CastToBP_Kyles_Character OtherActor))
  (Variables|/Game/Designers/Kyle/BP_Character/BP_Kyles_Character.BP_Kyles_Character_C|SetLocalChestRef _asbp_kyles_character self)
  (Variables|Default|SetIsLocal true))

(event OnComponentEndOverlap(ChestCollider)
  (params (OverlappedComponent :type Primitive%20Component%20Object%20Reference) (OtherActor :type Actor%20Object%20Reference) (OtherComp :type Primitive%20Component%20Object%20Reference) (OtherBodyIndex :type Integer))
  (bind _asbp_kyles_character (Utilities|Casting|CastToBP_Kyles_Character OtherActor))
  (Variables|/Game/Designers/Kyle/BP_Character/BP_Kyles_Character.BP_Kyles_Character_C|SetLocalChestRef _asbp_kyles_character self)
  (Variables|Default|SetIsLocal false))

(event Custom|Interact%20With%20Chest
  (if (Variables|Default|GetIsLocal)
    (switch Utilities|FlowControl|Switch|SwitchonE_ChestItems (Variables|Default|GetEnumItemOptions)
      (:NewEnumerator0
        (Default|AddShell (stale OnComponentBeginOverlap(ChestCollider) _asbp_kyles_character) (Variables|Default|GetBlueShellID)))
      (:NewEnumerator1
        (Default|AddShell (stale OnComponentBeginOverlap(ChestCollider) _asbp_kyles_character) (Variables|Default|GetRedShellID)))
      (:NewEnumerator2
        (Default|AddShell (stale OnComponentBeginOverlap(ChestCollider) _asbp_kyles_character) (Variables|Default|GetGreenShellID))))))

(fn ConstructionScript)