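; BP_Checkpoint is a shrine checkpoint that sets the player character's respawn location.
; Its trigger overlap caches the BP_Kyles_Character and sets IsLocal.
; InteractWithShrine, when IsLocal is set, passes the RespawnLocation1 component's world location to that cached character.
; End overlap also sets IsLocal to true, so the flag and cached character persist after leaving the trigger.
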(event OnComponentBeginOverlap(CheckpointTrigger)
  (params (OverlappedComponent :type Primitive%20Component%20Object%20Reference) (OtherActor :type Actor%20Object%20Reference) (OtherComp :type Primitive%20Component%20Object%20Reference) (OtherBodyIndex :type Integer) (bFromSweep :type Boolean) (SweepResult :type Hit%20Result%20Structure%20%28by%20ref%29))
  (bind _asbp_kyles_character (Utilities|Casting|CastToBP_Kyles_Character OtherActor))
  (Variables|Default|SetAs%20BP%20Kyles%20Character _asbp_kyles_character)
  (Variables|Default|SetIsLocal true))

(event OnComponentEndOverlap(CheckpointTrigger)
  (params (OverlappedComponent :type Primitive%20Component%20Object%20Reference) (OtherActor :type Actor%20Object%20Reference) (OtherComp :type Primitive%20Component%20Object%20Reference) (OtherBodyIndex :type Integer))
  (Utilities|Casting|CastToBP_Kyles_Character OtherActor)
  (Variables|Default|SetIsLocal true))

(event Custom|Interact%20With%20Shrine
  (if (Variables|Default|GetIsLocal)
    (Default|SetRespawnLocation (Variables|Default|GetAs%20BP%20Kyles%20Character) (Transformation|GetWorldLocation (Variables|Default|GetRespawnLocation1)))))

(fn ConstructionScript)