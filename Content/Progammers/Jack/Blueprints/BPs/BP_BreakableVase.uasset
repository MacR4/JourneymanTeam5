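; BP_BreakableVase is a Geometry Collection vase that a nearby player can break, counting towards tracked interactions.
; Sphere overlap registers the vase as the Kyles character's LocalJarRef and updates objective info.
; BreakJar fires once until reset, spawning a BP_Projectile at the player to break the vase and recording the interaction.
; The Chaos break event removes the sphere, disables debris collision after a delay, then destroys the actor.
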(event OnComponentBeginOverlap(Sphere)
  (params (OverlappedComponent :type Primitive%20Component%20Object%20Reference) (OtherActor :type Actor%20Object%20Reference) (OtherComp :type Primitive%20Component%20Object%20Reference) (OtherBodyIndex :type Integer) (bFromSweep :type Boolean) (SweepResult :type Hit%20Result%20Structure%20%28by%20ref%29))
  ;[0.4542 0.8796 1] Is Local checks
  (bind _asbp_kyles_character (Utilities|Casting|CastToBP_Kyles_Character OtherActor))
  (Variables|Default|SetPlayer _asbp_kyles_character)
  (Variables|Default|SetIsLocal true)
  (Variables|/Game/Designers/Kyle/BP_Character/BP_Kyles_Character.BP_Kyles_Character_C|SetLocalJarRef _asbp_kyles_character self)
  (bind _output_get (Variables|Default|SetKeyString (Utilities|String|EnumtoString (Variables|Default|GetKey))))
  (CallFunction|UpdateOBJInfo (Variables|Default|GetObj%20Info%20Text) true (Variables|Default|GetMax%20Num%20Interactions) _output_get))

(event OnChaosBreakEvent(Object_GC)
  (params (BreakEvent :type Chaos%20Break%20Event%20Structure%20%28by%20ref%29))
  (bind _player (Variables|Default|GetPlayer))
  ;[0.4937 1 0.6909] Object broken
  (Utilities|FlowControl|DoOnce false
    (:Completed
      (Components|DestroyComponent (Variables|Default|GetSphere))
      (Utilities|FlowControl|Delay (Variables|Default|GetCollision%20Delay))
      (Collision|SetCollisionEnabled (Variables|Default|GetObject_GC) "NoCollision")
      (Utilities|FlowControl|Delay 1.5)
      (Utilities|FlowControl|Sequence
        (:then_0
          (Actor|DestroyActor))
        (:then_1
          (Utilities|IsValid _player
            (:Is%20Valid
              (Variables|/Game/Designers/Kyle/BP_Character/BP_Kyles_Character.BP_Kyles_Character_C|SetLocalJarRef _player 0))))))))

(event OnComponentEndOverlap(Sphere)
  (params (OverlappedComponent :type Primitive%20Component%20Object%20Reference) (OtherActor :type Actor%20Object%20Reference) (OtherComp :type Primitive%20Component%20Object%20Reference) (OtherBodyIndex :type Integer))
  ;[0.4542 0.8796 1] Is Local checks
  (Utilities|Casting|CastToBP_Kyles_Character OtherActor)
  (Variables|Default|SetIsLocal false)
  (Utilities|FlowControl|Delay 0.2)
  (Variables|/Game/Designers/Kyle/BP_Character/BP_Kyles_Character.BP_Kyles_Character_C|SetLocalJarRef (Variables|Default|GetPlayer) 0))

(event Custom|BreakJar
  (bind _player (Variables|Default|GetPlayer))
  ;[0.8021 0.12 1] Make Object break
  (Utilities|FlowControl|DoOnce false
    (:Completed
      (if (Variables|Default|GetIsLocal)
        (Utilities|IsValid _player
          (:Is%20Valid
            (bind _returnvalue (Game|SpawnActorfromClass "/Game/Progammers/Jack/Blueprints/BPs/BP_Projectile.BP_Projectile_C" (Transformation|GetActorTransform _player) "Undefined" "MultiplyWithRoot" _player 0))
            (Default|BreakJar _returnvalue)
            (CallFunction|AddtoInteractions (Variables|Default|GetMax%20Num%20Interactions) (Variables|Default|GetKeyString) _player)))))))

(event Custom|ResetDoOnce
  (bind _player (Variables|Default|GetPlayer))
  ;[0.8021 0.12 1] Make Object break
  (Utilities|FlowControl|DoOnce false) ; enters at Reset
)

(event EventBeginPlay)

(fn ConstructionScript)