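; BP_Ladder is a ladder actor that moves the player character up or down along its PlayerPathway spline.
; Colliders for up and down cache the overlapping BP_Kyles_Character and set direction flags; only the up collider assigns the character's LocalLadderRef.
; PlayerUseLadder checks those flags, then runs chained timelines: one lerps the character to the relevant spline end, the next slides it along to the other end.
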(event OnComponentBeginOverlap(LadderColliderUp)
  (params (OverlappedComponent :type Primitive%20Component%20Object%20Reference) (OtherActor :type Actor%20Object%20Reference) (OtherComp :type Primitive%20Component%20Object%20Reference) (OtherBodyIndex :type Integer) (bFromSweep :type Boolean) (SweepResult :type Hit%20Result%20Structure%20%28by%20ref%29))
  ;[0.3183 1 0.3354] Collision Logic Up
  (bind _asbp_kyles_character (Utilities|Casting|CastToBP_Kyles_Character OtherActor))
  (Variables|Default|SetAs%20BP%20Kyles%20Character _asbp_kyles_character)
  (Variables|Default|SetIsLocalUp true)
  (Variables|/Game/Designers/Kyle/BP_Character/BP_Kyles_Character.BP_Kyles_Character_C|SetLocalLadderRef _asbp_kyles_character self))

(event OnComponentBeginOverlap(LadderColliderDown)
  (params (OverlappedComponent :type Primitive%20Component%20Object%20Reference) (OtherActor :type Actor%20Object%20Reference) (OtherComp :type Primitive%20Component%20Object%20Reference) (OtherBodyIndex :type Integer) (bFromSweep :type Boolean) (SweepResult :type Hit%20Result%20Structure%20%28by%20ref%29))
  ;[1 0.3194 0.2975] Collision Logic Down
  (bind _asbp_kyles_character (Utilities|Casting|CastToBP_Kyles_Character OtherActor))
  (Variables|Default|SetAs%20BP%20Kyles%20Character _asbp_kyles_character)
  (Variables|Default|SetIsLocalDown true))

(event OnComponentEndOverlap(LadderColliderUp)
  (params (OverlappedComponent :type Primitive%20Component%20Object%20Reference) (OtherActor :type Actor%20Object%20Reference) (OtherComp :type Primitive%20Component%20Object%20Reference) (OtherBodyIndex :type Integer))
  ;[0.3183 1 0.3354] Collision Logic Up
  (Variables|Default|SetIsLocalUp false))

(event OnComponentEndOverlap(LadderColliderDown)
  (params (OverlappedComponent :type Primitive%20Component%20Object%20Reference) (OtherActor :type Actor%20Object%20Reference) (OtherComp :type Primitive%20Component%20Object%20Reference) (OtherBodyIndex :type Integer))
  ;[1 0.3194 0.2975] Collision Logic Down
  (Variables|Default|SetIsLocalDown false))

(event Custom|PlayerUseLadder
  (bind _as_bp_kyles_character (Variables|Default|GetAs%20BP%20Kyles%20Character))
  (bind _as_bp_kyles_character_2 (Variables|Default|GetAs%20BP%20Kyles%20Character))
  (bind _playerpathway (Variables|Default|GetPlayerPathway))
  (bind _returnvalue (Spline|GetSplineLength _playerpathway))
  ;[1 1 1] Interact Input
  (Utilities|FlowControl|Sequence
    (:then_0
      ;[0.3216 1 0.2455] Move Player Up
      (if (Variables|Default|GetIsLocalUp)
        (bind _alpha (Timeline|Move%20To%20Spline%20Up PlayFromStart)
          (:Update
            (Transformation|SetActorLocation _as_bp_kyles_character (Math|Vector|Lerp(Vector) (Transformation|GetActorLocation _as_bp_kyles_character) (Spline|GetLocationatDistanceAlongSpline _playerpathway 0.0 "World") _alpha) false false))
          (:Finished
            (bind _alpha_2 (Timeline|Move%20Up%20Spline PlayFromStart)
              (:Update
                (Transformation|SetActorLocation (stale OnComponentBeginOverlap(LadderColliderUp) _asbp_kyles_character) (Spline|GetLocationatDistanceAlongSpline _playerpathway (Math|Float|Lerp 0.0 _returnvalue _alpha_2) "World") false false)))))))
    (:then_1
      ;[1 0.1195 0.1932] Move Player Down
      (if (Variables|Default|GetIsLocalDown)
        (bind _alpha_3 (Timeline|Move%20To%20Spline PlayFromStart)
          (:Update
            (Transformation|SetActorLocation _as_bp_kyles_character_2 (Math|Vector|Lerp(Vector) (Transformation|GetActorLocation _as_bp_kyles_character_2) (Spline|GetLocationatDistanceAlongSpline _playerpathway _returnvalue "World") _alpha_3) false false))
          (:Finished
            (bind _alpha_4 (Timeline|Move%20Down%20Spline PlayFromStart)
              (:Update
                (Transformation|SetActorLocation (stale OnComponentBeginOverlap(LadderColliderDown) _asbp_kyles_character) (Spline|GetLocationatDistanceAlongSpline _playerpathway (Math|Float|Lerp _returnvalue 0.0 _alpha_4) "World") false false)))))))))

(fn ConstructionScript)