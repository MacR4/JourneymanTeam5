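; BP_Checkpoint is a checkpoint actor that sets the respawn location of a BP_ThirdPersonCharacter.
; When the character enters CheckpointTrigger, it caches that character, sets IsLocal and immediately passes RespawnLocation1's world location to SetRespawnLoc.
; The IA_A input action repeats that save while IsLocal is true.
; End overlap also sets IsLocal to true, so the input keeps working after the character leaves.
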(event OnComponentBeginOverlap(CheckpointTrigger)
  (params (OverlappedComponent :type Primitive%20Component%20Object%20Reference) (OtherActor :type Actor%20Object%20Reference) (OtherComp :type Primitive%20Component%20Object%20Reference) (OtherBodyIndex :type Integer) (bFromSweep :type Boolean) (SweepResult :type Hit%20Result%20Structure%20%28by%20ref%29))
  (bind _asbp_third_person_character (Utilities|Casting|CastToBP_ThirdPersonCharacter OtherActor))
  (Variables|Default|SetThirdPerson _asbp_third_person_character)
  (Variables|Default|SetIsLocal true)
  (if (Variables|Default|GetIsLocal)
    (Default|SetRespawnLoc (Variables|Default|GetThirdPerson) (Transformation|GetWorldLocation (Variables|Default|GetRespawnLocation1)))))

(event OnComponentEndOverlap(CheckpointTrigger)
  (params (OverlappedComponent :type Primitive%20Component%20Object%20Reference) (OtherActor :type Actor%20Object%20Reference) (OtherComp :type Primitive%20Component%20Object%20Reference) (OtherBodyIndex :type Integer))
  (Utilities|Casting|CastToBP_ThirdPersonCharacter OtherActor)
  (Variables|Default|SetIsLocal true))

(event Input|EnhancedActionEvents|EnhancedInputActionIA_A
  (params (ActionValue :type Boolean) (ElapsedSeconds :type Float%20%28double-precision%29) (TriggeredSeconds :type Float%20%28double-precision%29) (InputAction :type Input%20Action%20Object%20Reference :default "/Game/General/ThirdPerson/Input/Actions/IA_A.IA_A"))
  (:Triggered
    (if (Variables|Default|GetIsLocal)
      (Default|SetRespawnLoc (Variables|Default|GetThirdPerson) (Transformation|GetWorldLocation (Variables|Default|GetRespawnLocation1))))))

(fn ConstructionScript)