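; BP_Platform_Mushroom is a mushroom platform that moves vertically toward EndHeight while the player is on it and back toward StartingHeight otherwise.
; Actor overlap events with BP_Kyles_Character set IsTouchingPlayer after a short delay.
; Tick compares the two heights to choose up or down, then offsets Z by Speed per frame without sweep, so movement is frame-rate dependent.
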(event Collision|EventActorBeginOverlap
  (params (OtherActor :type Actor%20Object%20Reference))
  ;[1 1 1] Moving Mushroom up and down
  ;;[1 1 1] Checking wether player is on mushroom
  (Utilities|Casting|CastToBP_Kyles_Character OtherActor)
  (Utilities|FlowControl|Delay 0.2)
  (Variables|Default|SetIs%20touching%20player? true))

(event EventTick
  (params (DeltaSeconds :type Float%20%28single-precision%29))
  (bind _returnvalue (Transformation|GetActorTransform))
  (bind _location (Math|Transform|BreakTransform _returnvalue))
  ;[1 1 1] Moving Mushroom up and down
  ;;[1 1 1] Set current location and height each tick
  (Variables|Default|SetCurrent%20Location _location)
  (Variables|Default|SetCurrent%20Height (.Z (Class|KismetMathLibrary|BreakVector3f _location)))
  (Variables|Default|SetEnd%20>%20Start (> (Variables|Default|GetEnd%20Height) (Variables|Default|GetStarting%20Height)))
  (if (Variables|Default|GetIs%20touching%20player?)
    (if (Variables|Default|GetEnd%20>%20Start)
      (if (<= (Variables|Default|GetCurrent%20Height) (Variables|Default|GetEnd%20Height))
        (Transformation|SetActorLocation (Math|Vector|MakeVector (.X (Class|KismetMathLibrary|BreakVector3f (Variables|Default|GetCurrent%20Location))) (.Y (Class|KismetMathLibrary|BreakVector3f (Variables|Default|GetCurrent%20Location))) (+ (.Z (Class|KismetMathLibrary|BreakVector3f (Variables|Default|GetCurrent%20Location))) (Variables|Default|GetSpeed))) false false))
      (elif (>= (Variables|Default|GetCurrent%20Height) (Variables|Default|GetEnd%20Height))
        (Transformation|SetActorLocation (Math|Vector|MakeVector (.X (Class|KismetMathLibrary|BreakVector3f (Variables|Default|GetCurrent%20Location))) (.Y (Class|KismetMathLibrary|BreakVector3f (Variables|Default|GetCurrent%20Location))) (- (.Z (Class|KismetMathLibrary|BreakVector3f (Variables|Default|GetCurrent%20Location))) (Variables|Default|GetSpeed))) false false)))
    (elif (Variables|Default|GetEnd%20>%20Start)
      (if (>= (Variables|Default|GetCurrent%20Height) (Variables|Default|GetStarting%20Height))
        (Transformation|SetActorLocation (Math|Vector|MakeVector (.X (Class|KismetMathLibrary|BreakVector3f (Variables|Default|GetCurrent%20Location))) (.Y (Class|KismetMathLibrary|BreakVector3f (Variables|Default|GetCurrent%20Location))) (- (.Z (Class|KismetMathLibrary|BreakVector3f (Variables|Default|GetCurrent%20Location))) (Variables|Default|GetSpeed))) false false))
      (elif (<= (Variables|Default|GetCurrent%20Height) (Variables|Default|GetStarting%20Height))
        (Transformation|SetActorLocation (Math|Vector|MakeVector (.X (Class|KismetMathLibrary|BreakVector3f (Variables|Default|GetCurrent%20Location))) (.Y (Class|KismetMathLibrary|BreakVector3f (Variables|Default|GetCurrent%20Location))) (+ (.Z (Class|KismetMathLibrary|BreakVector3f (Variables|Default|GetCurrent%20Location))) (Variables|Default|GetSpeed))) false false)))))

(event Collision|EventActorEndOverlap
  (params (OtherActor :type Actor%20Object%20Reference))
  ;[1 1 1] Moving Mushroom up and down
  ;;[1 1 1] Checking wether player is on mushroom
  (Utilities|Casting|CastToBP_Kyles_Character OtherActor)
  (Utilities|FlowControl|Delay 0.2)
  (Variables|Default|SetIs%20touching%20player? false))

(fn ConstructionScript)