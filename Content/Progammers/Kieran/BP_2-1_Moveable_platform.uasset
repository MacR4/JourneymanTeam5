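; Moveable platform Blueprint that the player character nudges along world X or Y through a universal interaction event.
; Overlapping actors that cast to BP_Kyles_Character are stored, and Tick caches the platform's location.
; Each interaction checks the Front, Left, Right and Back colliders in priority order, moving one unit without sweep.
; Front and Left drive opposite X directions, while Right and Back drive opposite Y directions.
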(event Input|EnhancedActionEvents|EnhancedInputActionIA_A
  (params (ActionValue :type Boolean) (ElapsedSeconds :type Float%20%28double-precision%29) (TriggeredSeconds :type Float%20%28double-precision%29) (InputAction :type Input%20Action%20Object%20Reference :default "/Game/General/ThirdPerson/Input/Actions/IA_A.IA_A")))

(event EventBeginPlay)

(event Collision|EventActorBeginOverlap
  (params (OtherActor :type Actor%20Object%20Reference))
  (bind _asbp_kyles_character (Utilities|Casting|CastToBP_Kyles_Character OtherActor))
  (Variables|Default|SetBP%20Kyles%20Character _asbp_kyles_character))

(event EventTick
  (params (DeltaSeconds :type Float%20%28single-precision%29))
  (Variables|Default|SetLocation (.Location (Math|Transform|BreakTransform (Transformation|GetActorTransform)))))

(event EventUniversalInteraction
  (bind _location (Variables|Default|GetLocation))
  (bind _location_2 (Variables|Default|GetLocation))
  (bind _location_3 (Variables|Default|GetLocation))
  (bind _location_4 (Variables|Default|GetLocation))
  (bind (_x _y _z) (Class|KismetMathLibrary|BreakVector3f _location_3))
  (bind (_x_2 _y_2 _z_2) (Class|KismetMathLibrary|BreakVector3f _location))
  (bind (_x_3 _y_3 _z_3) (Class|KismetMathLibrary|BreakVector3f _location_4))
  (bind (_x_4 _y_4 _z_4) (Class|KismetMathLibrary|BreakVector3f _location_2))
  (if (Collision|IsOverlappingActor (Variables|Default|GetFront%20Collider) (Variables|Default|GetBP%20Kyles%20Character) :!class /Script/Engine.PrimitiveComponent)
    (Transformation|SetActorLocation (Math|Vector|MakeVector (+ _x_2 1.0) _y_2 _z_2) false false)
    (elif (Collision|IsOverlappingActor (Variables|Default|GetLeft%20Collider) (Variables|Default|GetBP%20Kyles%20Character) :!class /Script/Engine.PrimitiveComponent)
      (Transformation|SetActorLocation (Math|Vector|MakeVector (- _x_4 1.0) _y_4 _z_4) false false)
      (elif (Collision|IsOverlappingActor (Variables|Default|GetRight%20Collider) (Variables|Default|GetBP%20Kyles%20Character) :!class /Script/Engine.PrimitiveComponent)
        (Transformation|SetActorLocation (Math|Vector|MakeVector _x (+ _y 1.0) _z) false false)
        (elif (Collision|IsOverlappingActor (Variables|Default|GetBack%20Collider) (Variables|Default|GetBP%20Kyles%20Character) :!class /Script/Engine.PrimitiveComponent)
          (Transformation|SetActorLocation (Math|Vector|MakeVector _x_3 (- _y_3 1.0) _z_3) false false))))))

(fn ConstructionScript)