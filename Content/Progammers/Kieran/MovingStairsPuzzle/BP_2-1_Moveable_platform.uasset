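; Pushable platform for the moving stairs puzzle that the player shoves along the world X or Y axis.
; Overlapping BP_Kyles_Character caches a reference to it.
; On UniversalInteraction, the first of the front, back, left or right colliders overlapping the player picks the direction.
; Platform and player are then both offset by PushSpeed per call via SetActorLocation without sweep, so the move ignores blocking collision.
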(event Collision|EventActorBeginOverlap
  (params (OtherActor :type Actor%20Object%20Reference))
  (bind _asbp_kyles_character (Utilities|Casting|CastToBP_Kyles_Character OtherActor))
  (Variables|Default|SetBP%20Kyles%20Character _asbp_kyles_character))

(event EventUniversalInteraction
  (Variables|Default|SetLocation (.Location (Math|Transform|BreakTransform (Transformation|GetActorTransform))))
  (Variables|Default|SetPlayer%20Location (.Location (Math|Transform|BreakTransform (Transformation|GetActorTransform (Variables|Default|GetBP%20Kyles%20Character)))))
  (if (Collision|IsOverlappingActor (Variables|Default|GetFront%20Collider) (Variables|Default|GetBP%20Kyles%20Character) :!class /Script/Engine.PrimitiveComponent)
    (Transformation|SetActorLocation (Math|Vector|MakeVector (+ (.X (Class|KismetMathLibrary|BreakVector3f (Variables|Default|GetLocation))) (Variables|Default|GetPush%20Speed)) (.Y (Class|KismetMathLibrary|BreakVector3f (Variables|Default|GetLocation))) (.Z (Class|KismetMathLibrary|BreakVector3f (Variables|Default|GetLocation)))) false false)
    (Transformation|SetActorLocation (Variables|Default|GetBP%20Kyles%20Character) (Math|Vector|MakeVector (+ (.X (Class|KismetMathLibrary|BreakVector3f (Variables|Default|GetPlayer%20Location))) (Variables|Default|GetPush%20Speed)) (.Y (Class|KismetMathLibrary|BreakVector3f (Variables|Default|GetPlayer%20Location))) (.Z (Class|KismetMathLibrary|BreakVector3f (Variables|Default|GetPlayer%20Location)))) false false)
    (elif (Collision|IsOverlappingActor (Variables|Default|GetBack%20Collider) (Variables|Default|GetBP%20Kyles%20Character) :!class /Script/Engine.PrimitiveComponent)
      (Transformation|SetActorLocation (Math|Vector|MakeVector (- (.X (Class|KismetMathLibrary|BreakVector3f (Variables|Default|GetLocation))) (Variables|Default|GetPush%20Speed)) (.Y (Class|KismetMathLibrary|BreakVector3f (Variables|Default|GetLocation))) (.Z (Class|KismetMathLibrary|BreakVector3f (Variables|Default|GetLocation)))) false false)
      (Transformation|SetActorLocation (Variables|Default|GetBP%20Kyles%20Character) (Math|Vector|MakeVector (- (.X (Class|KismetMathLibrary|BreakVector3f (Variables|Default|GetPlayer%20Location))) (Variables|Default|GetPush%20Speed)) (.Y (Class|KismetMathLibrary|BreakVector3f (Variables|Default|GetPlayer%20Location))) (.Z (Class|KismetMathLibrary|BreakVector3f (Variables|Default|GetPlayer%20Location)))) false false)
      (elif (Collision|IsOverlappingActor (Variables|Default|GetLeft%20Collider) (Variables|Default|GetBP%20Kyles%20Character) :!class /Script/Engine.PrimitiveComponent)
        (Transformation|SetActorLocation (Math|Vector|MakeVector (.X (Class|KismetMathLibrary|BreakVector3f (Variables|Default|GetLocation))) (+ (.Y (Class|KismetMathLibrary|BreakVector3f (Variables|Default|GetLocation))) (Variables|Default|GetPush%20Speed)) (.Z (Class|KismetMathLibrary|BreakVector3f (Variables|Default|GetLocation)))) false false)
        (Transformation|SetActorLocation (Variables|Default|GetBP%20Kyles%20Character) (Math|Vector|MakeVector (.X (Class|KismetMathLibrary|BreakVector3f (Variables|Default|GetPlayer%20Location))) (+ (.Y (Class|KismetMathLibrary|BreakVector3f (Variables|Default|GetPlayer%20Location))) (Variables|Default|GetPush%20Speed)) (.Z (Class|KismetMathLibrary|BreakVector3f (Variables|Default|GetPlayer%20Location)))) false false)
        (elif (Collision|IsOverlappingActor (Variables|Default|GetRight%20Collider) (Variables|Default|GetBP%20Kyles%20Character) :!class /Script/Engine.PrimitiveComponent)
          (Transformation|SetActorLocation (Math|Vector|MakeVector (.X (Class|KismetMathLibrary|BreakVector3f (Variables|Default|GetLocation))) (- (.Y (Class|KismetMathLibrary|BreakVector3f (Variables|Default|GetLocation))) (Variables|Default|GetPush%20Speed)) (.Z (Class|KismetMathLibrary|BreakVector3f (Variables|Default|GetLocation)))) false false)
          (Transformation|SetActorLocation (Variables|Default|GetBP%20Kyles%20Character) (Math|Vector|MakeVector (.X (Class|KismetMathLibrary|BreakVector3f (Variables|Default|GetPlayer%20Location))) (- (.Y (Class|KismetMathLibrary|BreakVector3f (Variables|Default|GetPlayer%20Location))) (Variables|Default|GetPush%20Speed)) (.Z (Class|KismetMathLibrary|BreakVector3f (Variables|Default|GetPlayer%20Location)))) false false))))))

(fn ConstructionScript)