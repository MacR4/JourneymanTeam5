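; Inventory component that holds a fixed-size array of item slots and lets its owning character interact with items.
; Each tick a forward sphere trace updates the look-at actor, which the Interact input sends through ServerInteract to its item data component.
; AddToInventory places units singly via FindSlot or empty slots, but FindSlot only matches negative quantities, so units never stack normally.
; Removal is empty and the data-table stack-size lookup is unused.
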(event Custom|Server_Interact
  (params (Target :type Actor%20Object%20Reference))
  (bind _returnvalue (Actor|GetComponentbyClass Target "/Game/Progammers/Tom/Blueprints/Inventory/Item_Data_Component.Item_Data_Component_C"))
  (Utilities|IsValid _returnvalue
    (:Is%20Valid
      (Class|IInteractInterface|Interactwith(Message) _returnvalue (.AsBP%20Third%20Person%20Character (Utilities|Casting|CastToBP_ThirdPersonCharacter (Components|GetOwner)))))))

(event EventBeginPlay
  (Utilities|Array|Resize (Variables|Default|GetContent) (Variables|Default|GetInventory_Size)))

(event EventTick
  (params (DeltaSeconds :type Float%20%28single-precision%29))
  (CallFunction|InteractionTrace))

(event Input|ActionEvents|InputActionInteract
  (params (Key :type Key%20Structure))
  (:Pressed
    (bind _look_at_actor (Variables|Default|Getlook_At_Actor)
      (:then
        (CallFunction|ServerInteract _look_at_actor))
      (:else))))

(fn AddtoInventory
  (params (ItemID :type Name) (Quantity :type Integer))
  (LocalVariables|SetLocal_Quantity_Remaining Quantity)
  (while (and (> (LocalVariables|GetLocal_Quantity_Remaining) 0) (not (LocalVariables|GetLocal_Has_Failed)))
    (bind (_index _foundslot) (CallFunction|FindSlot ItemID))
    (if _foundslot
      (CallFunction|AddtoStack _index 1)
      (Math|Integer|DecrementInt (LocalVariables|GetLocal_Quantity_Remaining))
      (elif (.Has_Empty_Slot (CallFunction|AnyEmptySlotsAvailable))
        (bind _success (CallFunction|CreateNewStack ItemID 1))
        (if _success
          (Math|Integer|DecrementInt (LocalVariables|GetLocal_Quantity_Remaining))
          (else
            (LocalVariables|SetLocal_Has_Failed true)))
        (else
          (LocalVariables|SetLocal_Has_Failed true)))))
  (return (not (LocalVariables|GetLocal_Has_Failed)) (LocalVariables|GetLocal_Quantity_Remaining)))

(fn RemovefromInventory)

(fn InteractionTrace
  (bind _returnvalue (Game|Player|GetPlayerPawn 0))
  (bind _returnvalue_2 (Transformation|GetActorLocation _returnvalue))
  (bind (_outhit _returnvalue_3) (Collision|SphereTraceByChannel _returnvalue_2 (+ _returnvalue_2 (* (Transformation|GetActorForwardVector _returnvalue) (Variables|Default|GetInteraction_Range))) 15.0 "TraceTypeQuery3" false (Utilities|Array|MakeArray (Components|GetOwner)) "None"))
  (if _returnvalue_3
    (if (!= (.HitActor (Collision|BreakHitResult _outhit)) (Variables|Default|Getlook_At_Actor))
      (bind _output_get (Variables|Default|Setlook_At_Actor (.HitActor (Collision|BreakHitResult _outhit))))
      (bind _message (Class|IInteractInterface|Lookat(Message) _output_get))
      (Development|PrintString (Utilities|String|ToString(Text) _message))
      (else
        (Variables|Default|Setlook_At_Actor 0)))))

(fn FindSlot
  (params (ItemID :type Name))
  (for (_array_element _array_index) (Variables|Default|GetContent)
    (if (== (.Item_ID (Utilities|Struct|BreakF_Slot_Structure _array_element)) ItemID)
      (if (< (.Quantity (Utilities|Struct|BreakF_Slot_Structure _array_element)) 0)
        (return _array_index true))))
  (return -1 false))

(fn GetMaxStackSize
  (params (ItemID :type Name))
  (bind _returnvalue (Utilities|GetDataTableRow "/Game/Progammers/Tom/Blueprints/Inventory/Item_Data.Item_Data" ItemID)
    (:then
      (return (Utilities|Struct|BreakF_Items_Structure _returnvalue)))
    (:RowNotFound
      (return -1))))

(fn AddtoStack
  (params (Index :type Integer) (Quantity :type Integer))
  (bind _content (Variables|Default|GetContent))
  (bind _output (Utilities|Array|Get(acopy) _content Index))
  (Utilities|Array|SetArrayElem (Variables|Default|GetContent) Index (Utilities|Struct|MakeF_Slot_Structure (.item_id _output) (+ (.quantity _output) Quantity))))

(fn AnyEmptySlotsAvailable
  (for (_array_element _array_index) (Variables|Default|GetContent)
    (if (== (.Quantity (Utilities|Struct|BreakF_Slot_Structure _array_element)) 0)
      (return true _array_index)))
  (return false -1))

(fn CreateNewStack
  (params (ItemID :type Name) (Quantity :type Integer))
  (bind (_has_empty_slot _empty_index) (CallFunction|AnyEmptySlotsAvailable))
  (if _has_empty_slot
    (Utilities|Array|SetArrayElem (Variables|Default|GetContent) _empty_index (Utilities|Struct|MakeF_Slot_Structure ItemID Quantity))
    (return true)
    (else
      (return false))))

(fn DebugPrintContents
  (for (_array_element _array_index) (Variables|Default|GetContent)
    (Development|PrintString (Utilities|String|Append (Utilities|String|ToString(Integer) _array_index) ":" (Utilities|String|ToString(Name) (.Item_ID (Utilities|Struct|BreakF_Slot_Structure _array_element))) "=" (Utilities|String|ToString(Integer) (.Quantity (Utilities|Struct|BreakF_Slot_Structure _array_element)))))))