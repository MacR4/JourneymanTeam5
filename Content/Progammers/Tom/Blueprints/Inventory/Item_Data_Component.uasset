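; Item data component that makes its owning actor a pickup the player can collect into their inventory.
; On BeginPlay it turns on replication for the owner.
; Interacting passes the item row name and quantity to the player's InventorySystem and destroys the owner if the add succeeds.
; Its LookAt function returns an empty string.
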(event EventInteractwith
  (params (Player_Character :type BP%20Third%20Person%20Character%20Object%20Reference))
  (bind _inventory_system (Variables|/Game/General/ThirdPerson/Blueprints/BP_ThirdPersonCharacter.BP_ThirdPersonCharacter_C|GetInventory_System Player_Character))
  (Utilities|IsValid _inventory_system
    (:Is%20Valid
      (bind _success (Default|AddtoInventory _inventory_system (.rowname (Variables|Default|GetItem_ID)) (Variables|Default|GetQuantity)))
      (if _success
        (Actor|DestroyActor (Components|GetOwner))))))

(event EventBeginPlay
  (Networking|SetReplicates (Components|GetOwner) true))

(fn Lookat
  (return ""))