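; BP_Health_Potion is an inventory item actor that heals the player when its Cube component registers a hit.
; The hit handler passes PlayerHealth to HealthPotion on player 0's BP_Kyles_Character, whatever caused the hit, then prints a message and destroys the actor.
; Its LookAt function looks up the item's data table row through ItemDataComponent and returns a "Pick Up" prompt with the item name.
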(event OnComponentHit(Cube)
  (params (HitComponent :type Primitive%20Component%20Object%20Reference) (OtherActor :type Actor%20Object%20Reference) (OtherComp :type Primitive%20Component%20Object%20Reference) (NormalImpulse :type Vector :default "0, 0, 0") (Hit :type Hit%20Result%20Structure%20%28by%20ref%29))
  (bind _asbp_kyles_character (Utilities|Casting|CastToBP_Kyles_Character (Game|GetPlayerCharacter 0)))
  (Default|HealthPotion _asbp_kyles_character (Variables|Default|GetPlayer_Health))
  (Development|PrintString "+ 15 Health")
  (Actor|DestroyActor))

(fn ConstructionScript)

(fn Lookat
  (bind _item_data_component (Variables|Default|GetItem_Data_Component))
  (bind _item_id (Variables|/Game/Progammers/Tom/Blueprints/Inventory/Item_Data_Component.Item_Data_Component_C|GetItem_ID _item_data_component))
  (bind _returnvalue (Utilities|GetDataTableRow (.datatable _item_id) (.rowname _item_id))
    (:then
      (return (Utilities|Text|FormatText "Pick Up {item}" (.Name (Utilities|Struct|BreakF_Items_Structure _returnvalue)))))))